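; Light switch actor that turns an array of linked light actors on or off, with matching switch sounds.
; A trigger box reacts to pawns, optionally switching lights on enter or leave, showing a text label, or enabling key control.
; While enabled, Tick polls the key and uses a DoOnce to toggle once per press.
; The construction script previews the initial light state and configures box size, emissive label and audio components.
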(event `self.ReceiveBeginPlay`
  (`SceneComponent.SetVisibility` (`self.TextRender`) false false)
  (`AudioComponent.Stop` (`self.Audio TurnOff Component`))
  (`AudioComponent.Stop` (`self.Audio TurnOn Component`))
  (for _array_element (`self.Lights`)
    (`/Engine/EditorBlueprintResources/StandardMacros.IsValid` _array_element
      (:`Is Valid`
        (set `/Game/InteractiveLights/Blueprints/BaseElements/Light_Base.Enabled` (`self.Switch On`) _array_element)
        (`/Game/InteractiveLights/Blueprints/BaseElements/Light_Base.Constructor` _array_element)))))

(event `self.ReceiveTick`
  (params (DeltaSeconds :type "Float (single-precision)"))
  (if (`self.Input Enabled`)
    (if (`PlayerController.IsInputKeyDown` (`GameplayStatics.GetPlayerController` 0) (`self.Key`))
      (`/Engine/EditorBlueprintResources/StandardMacros.DoOnce` true :!label _label
        (:`Completed`
          (if (`self.Switch On`)
            (`self.Switch Lights Off`)
            (else
              (`self.Switch Lights On`)))))
      (else
        (goto _label :!via `Reset`)))))

(event `Switch Lights On`
  (for _array_element (`self.Lights`)
    (`/Engine/EditorBlueprintResources/StandardMacros.IsValid` _array_element
      (:`Is Valid`
        (`/Game/InteractiveLights/Blueprints/BaseElements/Light_Base.Turn On` _array_element))))
  (set `self.Switch On` true)
  (`AudioComponent.Stop` (`self.Audio TurnOff Component`))
  (`AudioComponent.Play` (`self.Audio TurnOn Component`) 0.0))

(event `Switch Lights Off`
  (for _array_element (`self.Lights`)
    (`/Engine/EditorBlueprintResources/StandardMacros.IsValid` _array_element
      (:`Is Valid`
        (`/Game/InteractiveLights/Blueprints/BaseElements/Light_Base.Turn Off` _array_element))))
  (set `self.Switch On` false)
  (`AudioComponent.Stop` (`self.Audio TurnOn Component`))
  (`AudioComponent.Play` (`self.Audio TurnOff Component`) 0.0))

(event `self.Box.OnComponentBeginOverlap`
  (params (OverlappedComponent :type "PrimitiveComponent Object Reference") (OtherActor :type "Actor Object Reference") (OtherComp :type "PrimitiveComponent Object Reference") (OtherBodyIndex :type Integer) (bFromSweep :type Boolean) (SweepResult :type "HitResult Structure (by ref)"))
  (cast `Pawn` OtherActor)
  (if (`self.Lights Controled by Key`)
    (`self.EnableInput` (`GameplayStatics.GetPlayerController` 0))
    (set `self.Input Enabled` true))
  (if (`self.Lights On on Enter`)
    (`self.Switch Lights On`))
  (if (`self.Label Enabled`)
    (`SceneComponent.SetVisibility` (`self.TextRender`) true false)))

(event `self.Box.OnComponentEndOverlap`
  (params (OverlappedComponent :type "PrimitiveComponent Object Reference") (OtherActor :type "Actor Object Reference") (OtherComp :type "PrimitiveComponent Object Reference") (OtherBodyIndex :type Integer))
  (cast `Pawn` OtherActor)
  (if (`self.Lights Controled by Key`)
    (`self.DisableInput` (`GameplayStatics.GetPlayerController` 0))
    (set `self.Input Enabled` false))
  (if (`self.Lights Off on Leave`)
    (`self.Switch Lights Off`))
  (if (`self.Label Enabled`)
    (`SceneComponent.SetVisibility` (`self.TextRender`) false false)))

(fn `Setup Audio`
  (bind _returnvalue (`SceneComponent.GetRelativeTransform` (`self.Box`)))
  (`|ExecutionSequence`
    (:`then_0`
      (`/Engine/EditorBlueprintResources/StandardMacros.IsValid` (`self.Audio TurnOn Component`)
        (:`Is Valid`
          _)
        (:`Is Not Valid`
          (bind _returnvalue_2 (`AddComponent|NODE_AddAudioComponent-0` :`RelativeTransform` _returnvalue))
          (bind _output_get (set `self.Audio TurnOn Component` _returnvalue_2))))
      (`AudioComponent.SetSound` _output_get (`self.Switch On Sound`)))
    (:`then_1`
      (`/Engine/EditorBlueprintResources/StandardMacros.IsValid` (`self.Audio TurnOff Component`)
        (:`Is Valid`
          _)
        (:`Is Not Valid`
          (bind _returnvalue_3 (`AddComponent|NODE_AddAudioComponent-1` :`RelativeTransform` _returnvalue))
          (bind _output_get_2 (set `self.Audio TurnOff Component` _returnvalue_3))))
      (`AudioComponent.SetSound` _output_get_2 (`self.Switch Off Sound`)))
    (:`then_2`
      (`SceneComponent.SetVisibility` (`self.Audio TurnOn Component`) false true)
      (`SceneComponent.SetVisibility` (`self.Audio TurnOff Component`) false true))))

(fn `UserConstructionScript`
  (bind _textrender (`self.TextRender`))
  (for _array_element (`self.Lights`)
    (if (`self.Switch On`)
      (set `/Game/InteractiveLights/Blueprints/BaseElements/Light_Base.Enabled` true _array_element)
      (else
        (set `/Game/InteractiveLights/Blueprints/BaseElements/Light_Base.Enabled` false _array_element)))
    (`/Game/InteractiveLights/Blueprints/BaseElements/Light_Base.Constructor` _array_element))
  (`TextRenderComponent.K2_SetText` (`self.TextRender`) (`self.Text`))
  (`BoxComponent.SetBoxExtent` (`self.Box`) (`self.BoxExtent`) true)
  (`SceneComponent.SetVisibility` _textrender (`self.Label Enabled`) false)
  (if (not (`self.Use Text Default Position`))
    (`SceneComponent.K2_SetRelativeLocation` _textrender (`self.Text Position`) false false))
  (`TextRenderComponent.SetWorldSize` _textrender (`self.Text Size`))
  (bind _returnvalue (`PrimitiveComponent.CreateDynamicMaterialInstance` (`self.TextRender`) 0 "/Game/InteractiveLights/Materials/M_FontEmissve.M_FontEmissve"))
  (`MaterialInstanceDynamic.SetVectorParameterValue` _returnvalue "TextColor" (`self.TextColor`))
  (`self.Setup Audio`))