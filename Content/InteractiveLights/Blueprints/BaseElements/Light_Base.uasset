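; Base interactive light actor that switches on and off with optional timer delays, eased heat-up and cooldown, and switchable flicker or pulse behaviors.
; The construction script sets up the light, creates idle and switch audio components, and builds dynamic material instances for the mesh's emissive glow.
; Tick drives HeatUpPercentage, random interpolated flicker and phase-shifted cosine pulse, feeding light intensity, emissive strength and, in some modes optionally, idle volume.
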(event Custom|Turn%20Off
  (bind _switch_off_time_offset (Variables|LightControl|GetSwitch%20Off%20Time%20Offset))
  ;[1 0.7167 0.3841] Switch light on / off (handles timers and calls Lights On / Off functions)
  (if (or (and (Variables|Default|GetEnabled) (not (Class|KismetSystemLibrary|TimerExistsHandle (Variables|ControlVariables|GetTimerHandleOff)))) (Class|KismetSystemLibrary|TimerExistsHandle (Variables|ControlVariables|GetTimerHandleOn)))
    (if (Class|KismetSystemLibrary|TimerExistsHandle (Variables|ControlVariables|GetTimerHandleOn))
      (Utilities|Time|ClearandInvalidateTimerbyHandle (Variables|ControlVariables|GetTimerHandleOn)))
    (if (> _switch_off_time_offset 0.0)
      (bind _returnvalue (Utilities|Time|SetTimerbyFunctionName self "LightsOff" _switch_off_time_offset))
      (Variables|ControlVariables|SetTimerHandleOff _returnvalue)
      (else
        (CallFunction|LightsOff)))))

(event Custom|Start%20Pulse
  ;[0.3117 1 0.3016] Control functions for enabling / disabling diffrent light behaviour modifications
  (Variables|LightControl|SetLight%20Behavior "NewEnumerator2")
  (Variables|TemporaryVariables|SetTemp_Timer%20Pulse 0.0))

(event Custom|Start%20Flickering
  ;[0.3117 1 0.3016] Control functions for enabling / disabling diffrent light behaviour modifications
  (Variables|LightControl|SetLight%20Behavior "NewEnumerator1")
  (CallFunction|RecalculateFlickerVariables))

(event Custom|Turn%20On
  (bind _switch_on_time_offset (Variables|LightControl|GetSwitch%20On%20Time%20Offset))
  ;[1 0.7167 0.3841] Switch light on / off (handles timers and calls Lights On / Off functions)
  (if (or (and (not (Variables|Default|GetEnabled)) (not (Class|KismetSystemLibrary|TimerExistsHandle (Variables|ControlVariables|GetTimerHandleOn)))) (Class|KismetSystemLibrary|TimerExistsHandle (Variables|ControlVariables|GetTimerHandleOff)))
    (if (Class|KismetSystemLibrary|TimerExistsHandle (Variables|ControlVariables|GetTimerHandleOff))
      (Utilities|Time|ClearandInvalidateTimerbyHandle (Variables|ControlVariables|GetTimerHandleOff)))
    (if (> _switch_on_time_offset 0.0)
      (bind _returnvalue (Utilities|Time|SetTimerbyFunctionName self "LightsOn" _switch_on_time_offset))
      (Variables|ControlVariables|SetTimerHandleOn _returnvalue)
      (else
        (CallFunction|Lightson)))))

(event Custom|Stop%20Pulse
  ;[0.3117 1 0.3016] Control functions for enabling / disabling diffrent light behaviour modifications
  (Variables|LightControl|SetLight%20Behavior "NewEnumerator0")
  (if (not (Variables|ControlVariables|GetbIsChangingTemperature))
    (Rendering|Components|Light|SetIntensity (Variables|Default|GetLight) (Variables|LightControl|GetMax%20Intensity))
    (CallFunction|ChangeEmissiveValue 1.0)
    (if (Variables|Pulsing|GetModulate%20Sound%20Volume%20During%20Pulse)
      (Audio|Components|Audio|SetVolumeMultiplier (Variables|Default|GetAudio%20Idle%20Component) (Variables|ControlVariables|GetIdle%20Volume) :!class /Script/Engine.AudioComponent))))

(event Custom|Stop%20Flickering
  ;[0.3117 1 0.3016] Control functions for enabling / disabling diffrent light behaviour modifications
  (Variables|LightControl|SetLight%20Behavior "NewEnumerator0")
  (if (not (Variables|ControlVariables|GetbIsChangingTemperature))
    (Rendering|Components|Light|SetIntensity (Variables|Default|GetLight) (Variables|LightControl|GetMax%20Intensity))
    (CallFunction|ChangeEmissiveValue 1.0)
    (if (Variables|Flickering|GetModulate%20Sound%20Volume)
      (Audio|Components|Audio|SetVolumeMultiplier (Variables|Default|GetAudio%20Idle%20Component) (Variables|ControlVariables|GetIdle%20Volume) :!class /Script/Engine.AudioComponent))))

(event EventBeginPlay
  ;[0.7369 1 0.9617] Begin play
  (if (Variables|Default|GetEnabled)
    (Audio|Components|Audio|Stop (Variables|Default|GetAudio%20TurnOn%20Component))
    (else
      (Audio|Components|Audio|Stop (Variables|Default|GetAudio%20Idle%20Component)))))

(event EventTick
  (params (DeltaSeconds :type Float%20%28single-precision%29))
  ;[0.2659 0.3614 1] Heatup / cooldown / flicker / pulse control
  (if (Variables|ControlVariables|GetbIsChangingTemperature)
    (CallFunction|HeatupLamp (Variables|ControlVariables|GetIntensityChangeType) DeltaSeconds))
  (if (Variables|Default|GetEnabled)
    (CallFunction|Flicker DeltaSeconds)
    (CallFunction|Pulse DeltaSeconds)))

(fn ConstructionScript
  (CallFunction|Constructor))

(fn HeatupLamp
  (params (ChangeType :type LightOn_Off%20Enum :default "NewEnumerator0") (Delta%20Time :type Float%20%28single-precision%29))
  (bind _heatup_percentage (Variables|ControlVariables|GetHeatUp%20Percentage))
  (bind _light (Variables|Default|GetLight))
  (switch Utilities|FlowControl|Switch|SwitchonLightOn_Off ChangeType
    (:NewEnumerator0
      (CallFunction|CalculateHeatUpPercentage Delta%20Time (Variables|TemporaryVariables|GetTemp_SwitchOnDuration) 1.0)
      (if (Utilities|Enum|Equal(Enum) (Variables|LightControl|GetLight%20Behavior) "NewEnumerator0")
        (Rendering|Components|Light|SetIntensity _light (Math|Interpolation|Ease "ExpoOut" (Variables|ControlVariables|GetHeatUp%20Percentage) (Variables|LightControl|GetMin%20Intensity) (Variables|LightControl|GetMax%20Intensity)))
        (Audio|Components|Audio|SetVolumeMultiplier (Variables|Default|GetAudio%20Idle%20Component) (* (Variables|ControlVariables|GetIdle%20Volume) _heatup_percentage) :!class /Script/Engine.AudioComponent)
        (CallFunction|ChangeEmissiveValue _heatup_percentage :!label _label)))
    (:NewEnumerator1
      (CallFunction|CalculateHeatUpPercentage Delta%20Time (Variables|TemporaryVariables|GetTemp_SwitchOffDuration) 0.0)
      (Rendering|Components|Light|SetIntensity _light (Math|Interpolation|Ease "ExpoIn" (Variables|ControlVariables|GetHeatUp%20Percentage) 0.0 (Variables|LightControl|GetMax%20Intensity)))
      (goto _label))))

(fn PlaySwichonSounds
  (Audio|Components|Audio|Stop (Variables|Default|GetAudio%20TurnOff%20Component))
  (Audio|Components|Audio|Play (Variables|Default|GetAudio%20Idle%20Component) 0.0))

(fn PlaySwitchOffSounds
  (Audio|Components|Audio|Play (Variables|Default|GetAudio%20TurnOff%20Component) 0.0)
  (Audio|Components|Audio|Stop (Variables|Default|GetAudio%20Idle%20Component)))

(fn Flicker
  (params (Delta%20Time :type Float%20%28single-precision%29))
  (bind _light (Variables|Default|GetLight))
  (bind _temp_flicker_intensity (Variables|TemporaryVariables|GetTemp_Flicker%20Intensity))
  (bind _temp_maxintensity (Variables|TemporaryVariables|GetTemp_MaxIntensity))
  (bind _flicker_min_interval (Variables|Flickering|GetFlicker%20Min%20Interval))
  (bind _flicker_max_interval (Variables|Flickering|GetFlicker%20Max%20Interval))
  (bind _returnvalue (Math|Float|MapRangeClamped _flicker_min_interval 0.01 0.2 0.0 1.0))
  (bind _returnvalue_2 (Math|Float|MapRangeClamped _flicker_max_interval 0.1 0.5 0.0 1.0))
  (bind _intensity (Variables|/Script/Engine.LightComponentBase|GetIntensity _light))
  (bind _returnvalue_3 (Math|Float|Lerp 25.0 1.0 _returnvalue))
  (bind _returnvalue_4 (Math|Float|Lerp 5e+01 3.0 _returnvalue_2))
  (bind _returnvalue_5 (Math|Random|RandomFloatinRange _returnvalue_3 _returnvalue_4))
  (bind _returnvalue_6 (Math|Interpolation|FInterpTo _intensity _temp_flicker_intensity Delta%20Time _returnvalue_5))
  (bind _returnvalue_7 (/ _returnvalue_6 _temp_maxintensity))
  (if (Utilities|Enum|Equal(Enum) (Variables|LightControl|GetLight%20Behavior) "NewEnumerator1")
    (if (>= (Variables|TemporaryVariables|GetTemp_Flicker%20Interval) (Variables|TemporaryVariables|GetTemp_Timer%20Flicker))
      (Rendering|Components|Light|SetIntensity _light _returnvalue_6)
      (CallFunction|ChangeEmissiveValue _returnvalue_7)
      (Variables|TemporaryVariables|SetTemp_Timer%20Flicker (+ (Variables|TemporaryVariables|GetTemp_Timer%20Flicker) Delta%20Time))
      (if (Variables|Flickering|GetModulate%20Sound%20Volume)
        (Audio|Components|Audio|SetVolumeMultiplier (Variables|Default|GetAudio%20Idle%20Component) (* (Variables|ControlVariables|GetIdle%20Volume) _returnvalue_7) :!class /Script/Engine.AudioComponent))
      (else
        (CallFunction|RecalculateFlickerVariables)))))

(fn RecalculateFlickerVariables
  (bind _heatup_percentage (Variables|ControlVariables|GetHeatUp%20Percentage))
  (CallFunction|RecalculateMaxIntensity)
  (Variables|TemporaryVariables|SetTemp_Flicker%20Interval (Math|Random|RandomFloatinRange (Variables|Flickering|GetFlicker%20Min%20Interval) (Variables|Flickering|GetFlicker%20Max%20Interval)))
  (Variables|TemporaryVariables|SetTemp_Flicker%20Intensity (Math|Random|RandomFloatinRange (* (Variables|LightControl|GetMin%20Intensity) _heatup_percentage) (* _heatup_percentage (Variables|TemporaryVariables|GetTemp_MaxIntensity))))
  (Variables|TemporaryVariables|SetTemp_Timer%20Flicker 0.0))

(fn SetupSoundSystem
  (bind _light (Variables|Default|GetLight))
  (bind _returnvalue (Transformation|GetRelativeTransform _light))
  (Utilities|FlowControl|Sequence
    (:then_0
      (Utilities|IsValid (Variables|Default|GetAudio%20Idle%20Component)
        (:Is%20Valid
          _)
        (:Is%20Not%20Valid
          (bind _returnvalue_2 (AddComponent|AddAudioComponent false _returnvalue))
          (bind _output_get (Variables|Default|SetAudio%20Idle%20Component _returnvalue_2))))
      (Audio|Components|Audio|SetSound _output_get (Variables|Sounds|GetIdle%20Sound)))
    (:then_1
      (Utilities|IsValid (Variables|Default|GetAudio%20TurnOn%20Component)
        (:Is%20Valid
          _)
        (:Is%20Not%20Valid
          (bind _returnvalue_3 (AddComponent|AddAudioComponent false _returnvalue))
          (bind _output_get_2 (Variables|Default|SetAudio%20TurnOn%20Component _returnvalue_3))))
      (Audio|Components|Audio|SetSound _output_get_2 (Variables|Sounds|GetLight%20Switch%20On%20Sound)))
    (:then_2
      (Utilities|IsValid (Variables|Default|GetAudio%20TurnOff%20Component)
        (:Is%20Valid
          _)
        (:Is%20Not%20Valid
          (bind _returnvalue_4 (AddComponent|AddAudioComponent false _returnvalue))
          (bind _output_get_3 (Variables|Default|SetAudio%20TurnOff%20Component _returnvalue_4))))
      (Audio|Components|Audio|SetSound _output_get_3 (Variables|Sounds|GetLight%20Switch%20Off%20Sound)))
    (:then_3
      (Variables|ControlVariables|SetIdle%20Volume (Variables|/Script/Engine.AudioComponent|GetVolumeMultiplier (Variables|Default|GetAudio%20Idle%20Component)))
      (Rendering|SetVisibility (Variables|Default|GetAudio%20Idle%20Component) false true))))

(fn Pulse
  (params (DeltaTime :type Float%20%28single-precision%29))
  (bind _pulse_duration (Variables|Pulsing|GetPulse%20Duration))
  (bind _heatup_percentage (Variables|ControlVariables|GetHeatUp%20Percentage))
  (if (Utilities|Enum|Equal(Enum) (Variables|LightControl|GetLight%20Behavior) "NewEnumerator2")
    (if (> _pulse_duration (Variables|TemporaryVariables|GetTemp_Timer%20Pulse))
      (CallFunction|RecalculateMaxIntensity)
      (Rendering|Components|Light|SetIntensity (Variables|Default|GetLight) (Math|Float|Lerp (* (Variables|LightControl|GetMin%20Intensity) _heatup_percentage) (* _heatup_percentage (Variables|TemporaryVariables|GetTemp_MaxIntensity)) (Math|Float|NormalizetoRange (Math|Trig|Cos(Degrees) (Math|Float|MapRangeUnclamped (|((TempTimer+Offset)%Duration) (Variables|TemporaryVariables|GetTemp_Timer%20Pulse) (Math|Float|Lerp 0.0 _pulse_duration (Variables|Pulsing|GetPhase%20Shift)) _pulse_duration) 0.0 _pulse_duration 0.0 3.6e+02)) -1.0 1.0)))
      (Variables|TemporaryVariables|SetTemp_Timer%20Pulse (+ (Variables|TemporaryVariables|GetTemp_Timer%20Pulse) DeltaTime))
      (CallFunction|ChangeEmissiveValue (/ (Math|Float|Lerp (* (Variables|LightControl|GetMin%20Intensity) _heatup_percentage) (* _heatup_percentage (Variables|TemporaryVariables|GetTemp_MaxIntensity)) (Math|Float|NormalizetoRange (Math|Trig|Cos(Degrees) (Math|Float|MapRangeUnclamped (|((TempTimer+Offset)%Duration) (Variables|TemporaryVariables|GetTemp_Timer%20Pulse) (Math|Float|Lerp 0.0 _pulse_duration (Variables|Pulsing|GetPhase%20Shift)) _pulse_duration) 0.0 _pulse_duration 0.0 3.6e+02)) -1.0 1.0)) (Variables|TemporaryVariables|GetTemp_MaxIntensity)))
      (if (Variables|Pulsing|GetModulate%20Sound%20Volume%20During%20Pulse)
        (Audio|Components|Audio|SetVolumeMultiplier (Variables|Default|GetAudio%20Idle%20Component) (* (Variables|ControlVariables|GetIdle%20Volume) (Variables|ControlVariables|GetHeatUp%20Percentage)) :!class /Script/Engine.AudioComponent))
      (else
        (Variables|TemporaryVariables|SetTemp_Timer%20Pulse 0.0)))))

(fn ChangeEmissiveValue
  (params (EmissivePercentage :type Float%20%28single-precision%29))
  (for _array_element (Variables|ControlVariables|GetMIDs)
    (Rendering|Material|SetScalarParameterValue _array_element (Variables|ControlVariables|GetEmissiveScalarParamName) (* (Variables|LightControl|GetILS_Emissive) (Math|Float|Clamp(Float) EmissivePercentage)) :!class /Script/Engine.MaterialInstanceDynamic)))

(fn Constructor
  (bind _light (Variables|Default|GetLight))
  (Utilities|IsValid (Variables|Default|GetLight)
    (:Is%20Valid
      (Utilities|Array|Clear (Variables|ControlVariables|GetMIDs))
      (if (Variables|Default|GetEnabled)
        (Variables|ControlVariables|SetHeatUp%20Percentage 1.0)
        (Rendering|Components|Light|SetIntensity _light (Variables|LightControl|GetMax%20Intensity))
        (else
          (Variables|ControlVariables|SetHeatUp%20Percentage 0.0)
          (Rendering|Components|Light|SetIntensity _light 0.0)))
      (Rendering|Components|Light|SetLightColor _light (Variables|LightControl|GetLight%20Color) true)
      (Variables|ControlVariables|SetbIsChangingTemperature false)
      (if (Variables|Default|GetUse%20Default%20Position)
        _
        (else
          (Transformation|SetRelativeLocation (Variables|Default|GetLight) (Variables|Default|GetLight%20Position) false false)))
      (CallFunction|SetupSoundSystem)
      (for _index (range 0 (- (Rendering|Material|GetNumMaterials (Variables|Debug|GetStaticMeshComponent)) 1))
        (bind _returnvalue (Rendering|Material|CreateDynamicMaterialInstance (Variables|Debug|GetStaticMeshComponent) _index 0 :!class /Script/Engine.PrimitiveComponent))
        (Utilities|Array|Add (Variables|ControlVariables|GetMIDs) _returnvalue)
        (if (Variables|Default|GetEnabled)
          (Rendering|Material|SetScalarParameterValue _returnvalue (Variables|ControlVariables|GetEmissiveScalarParamName) (Variables|LightControl|GetILS_Emissive) :!class /Script/Engine.MaterialInstanceDynamic)
          (else
            (Rendering|Material|SetScalarParameterValue _returnvalue (Variables|ControlVariables|GetEmissiveScalarParamName) 0.0 :!class /Script/Engine.MaterialInstanceDynamic)))
        (Rendering|Material|SetVectorParameterValue _returnvalue (Variables|ControlVariables|GetEmissiveVectorParamName) (Variables|LightControl|GetLight%20Color) :!class /Script/Engine.MaterialInstanceDynamic))
      (switch Utilities|FlowControl|Switch|SwitchonLightModification (Variables|LightControl|GetLight%20Behavior)
        (:NewEnumerator1
          (CallFunction|RecalculateFlickerVariables))
        (:NewEnumerator2
          (Variables|TemporaryVariables|SetTemp_Timer%20Pulse 0.0))))))

(fn CalculateHeatUpPercentage
  (params (Time :type Float%20%28single-precision%29) (Duration :type Float%20%28single-precision%29) (Range :type Float%20%28single-precision%29))
  (Variables|TemporaryVariables|SetTemp_Timer%20Change%20Intensity (+ Time (Variables|TemporaryVariables|GetTemp_Timer%20Change%20Intensity)))
  (Variables|ControlVariables|SetHeatUp%20Percentage (Math|Float|MapRangeClamped (Variables|TemporaryVariables|GetTemp_Timer%20Change%20Intensity) 0.0 Duration (Variables|TemporaryVariables|GetTemp_HeatUpPercent) Range))
  (Variables|ControlVariables|SetbIsChangingTemperature (not (>= (Variables|TemporaryVariables|GetTemp_Timer%20Change%20Intensity) Duration))))

(fn Lightson
  (bind _light (Variables|Default|GetLight))
  (bind _heatup_time (Variables|LightControl|GetHeatup%20Time))
  (bind _light_2 (Variables|Default|GetLight))
  (if (not (Variables|Default|GetEnabled))
    (if (== (Variables|LightControl|GetHeatup%20Time) 0.0)
      (if (or (Utilities|Enum|Equal(Enum) (Variables|LightControl|GetLight%20Behavior) "NewEnumerator2") (Utilities|Enum|Equal(Enum) (Variables|LightControl|GetLight%20Behavior) "NewEnumerator1"))
        (if (Variables|ControlVariables|GetbIsChangingTemperature)
          (Rendering|Components|Light|SetIntensity _light_2 (Variables|/Script/Engine.LightComponentBase|GetIntensity _light_2))
          (else
            (Rendering|Components|Light|SetIntensity _light_2 0.0)))
        (else
          (Rendering|Components|Light|SetIntensity _light (Variables|LightControl|GetMax%20Intensity))))
      (Variables|ControlVariables|SetHeatUp%20Percentage 1.0)
      (Variables|ControlVariables|SetbIsChangingTemperature false)
      (for _array_element (Variables|ControlVariables|GetMIDs)
        (Rendering|Material|SetScalarParameterValue _array_element (Variables|ControlVariables|GetEmissiveScalarParamName) (Variables|LightControl|GetILS_Emissive) :!class /Script/Engine.MaterialInstanceDynamic))
      (Variables|Default|SetEnabled true)
      (Audio|Components|Audio|SetVolumeMultiplier (Variables|Default|GetAudio%20Idle%20Component) (Variables|ControlVariables|GetIdle%20Volume) :!class /Script/Engine.AudioComponent)
      (else
        (if (Variables|ControlVariables|GetbIsChangingTemperature)
          (Variables|TemporaryVariables|SetTemp_SwitchOnDuration (- _heatup_time (* (Variables|ControlVariables|GetHeatUp%20Percentage) _heatup_time)))
          (else
            (Rendering|Components|Light|SetIntensity _light (Variables|LightControl|GetMin%20Intensity))
            (Variables|ControlVariables|SetbIsChangingTemperature true)
            (Variables|TemporaryVariables|SetTemp_SwitchOnDuration _heatup_time)))
        (Variables|TemporaryVariables|SetTemp_HeatUpPercent (Variables|ControlVariables|GetHeatUp%20Percentage))
        (Variables|ControlVariables|SetIntensityChangeType "NewEnumerator0")
        (Variables|TemporaryVariables|SetTemp_Timer%20Change%20Intensity 0.0)
        (Variables|Default|SetEnabled true)))
    (CallFunction|PlaySwichonSounds)
    (switch Utilities|FlowControl|Switch|SwitchonLightModification (Variables|LightControl|GetLight%20Behavior)
      (:NewEnumerator1
        (CallFunction|RecalculateFlickerVariables))
      (:NewEnumerator2
        (Variables|TemporaryVariables|SetTemp_Timer%20Pulse 0.0)))))

(fn LightsOff
  (bind _light_behavior (Variables|LightControl|GetLight%20Behavior))
  (bind _cooldown_time (Variables|LightControl|GetCooldown%20Time))
  (bind _light (Variables|Default|GetLight))
  (if (Variables|Default|GetEnabled)
    (if (== (Variables|LightControl|GetCooldown%20Time) 0.0)
      (Rendering|Components|Light|SetIntensity _light 0.0)
      (Variables|ControlVariables|SetbIsChangingTemperature false)
      (Variables|ControlVariables|SetHeatUp%20Percentage 0.0)
      (for _array_element (Variables|ControlVariables|GetMIDs)
        (Rendering|Material|SetScalarParameterValue _array_element (Variables|ControlVariables|GetEmissiveScalarParamName) 0.0 :!class /Script/Engine.MaterialInstanceDynamic))
      (else
        (Variables|ControlVariables|SetbIsChangingTemperature true)
        (Variables|ControlVariables|SetIntensityChangeType "NewEnumerator1")
        (Variables|TemporaryVariables|SetTemp_Timer%20Change%20Intensity 0.0)
        (if (or (Utilities|Enum|Equal(Enum) _light_behavior "NewEnumerator1") (Utilities|Enum|Equal(Enum) _light_behavior "NewEnumerator2"))
          (Variables|ControlVariables|SetHeatUp%20Percentage (/ (Variables|/Script/Engine.LightComponentBase|GetIntensity _light) (Variables|LightControl|GetMax%20Intensity))))
        (if (< (Variables|ControlVariables|GetHeatUp%20Percentage) 1.0)
          (Variables|TemporaryVariables|SetTemp_SwitchOffDuration (* (Variables|ControlVariables|GetHeatUp%20Percentage) _cooldown_time))
          (else
            (Variables|TemporaryVariables|SetTemp_SwitchOffDuration _cooldown_time)))
        (Variables|TemporaryVariables|SetTemp_HeatUpPercent (Variables|ControlVariables|GetHeatUp%20Percentage))))
    (CallFunction|PlaySwitchOffSounds)
    (Variables|Default|SetEnabled false)))

(fn RecalculateMaxIntensity
  (if (and (== (Variables|LightControl|GetMax%20Intensity) 0.0) (== (Variables|LightControl|GetMin%20Intensity) 0.0))
    (Variables|TemporaryVariables|SetTemp_MaxIntensity (Variables|LightControl|GetILS_Emissive))
    (else
      (Variables|TemporaryVariables|SetTemp_MaxIntensity (Variables|LightControl|GetMax%20Intensity)))))