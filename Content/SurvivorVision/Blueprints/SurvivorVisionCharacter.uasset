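; Player character for a Survivor Vision feature, carrying the detection sphere, distortion sphere and post-process components the effect uses.
; It forwards detection-sphere begin and end overlaps to a stored player controller as OverlapMessage calls with an Off flag, once that controller is set through SetController.
; Getter functions expose the mesh, camera and Survivor Vision components, leaving the vision logic outside this Blueprint.
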(event `/Game/SurvivorVision/Blueprints/BPInt_SurvivorVision_Character.SetController`
  (params (Controller :type "PlayerController Object Reference"))
  (set `self.PlayerController` Controller))

(event `self.SV_DetectionSphere.OnComponentBeginOverlap`
  (params (OtherActor :type "Actor Object Reference") (OtherComp :type "PrimitiveComponent Object Reference") (OtherBodyIndex :type Integer) (bFromSweep :type Boolean) (SweepResult :type "HitResult Structure (by ref)"))
  (`/Engine/EditorBlueprintResources/StandardMacros.IsValid` (`self.PlayerController`)
    (:`Is Valid`
      (message `/Game/SurvivorVision/Blueprints/BPInt_SurvivorVision_Controller.Overlap` (`self.PlayerController`) false OtherActor))))

(event `self.SV_DetectionSphere.OnComponentEndOverlap`
  (params (OtherActor :type "Actor Object Reference") (OtherComp :type "PrimitiveComponent Object Reference") (OtherBodyIndex :type Integer))
  (`/Engine/EditorBlueprintResources/StandardMacros.IsValid` (`self.PlayerController`)
    (:`Is Valid`
      (message `/Game/SurvivorVision/Blueprints/BPInt_SurvivorVision_Controller.Overlap` (`self.PlayerController`) true OtherActor))))

(fn `GetCharacterMesh`
  (returns (Mesh :type "SkeletalMeshComponent Object Reference"))
  (return (`self.Mesh`)))

(fn `GetPlayerCamera`
  (returns (Camera :type "CameraComponent Object Reference"))
  (return (`self.Camera`)))

(fn `GetSVComponents`
  (returns (SVPostProcess :type "PostProcessComponent Object Reference") (SVDistortionSphere :type "StaticMeshComponent Object Reference") (SVDetectionSphere :type "SphereComponent Object Reference"))
  (return (`self.SV_PostProcess`) (`self.SV_DistortionSphere`) (`self.SV_DetectionSphere`)))

(fn `UserConstructionScript`)