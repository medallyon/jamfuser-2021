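; BP_EasyFollowTarget is a spline waypoint actor that walks a referenced AI character along its points, with optional waiting for the player.
; A Loop timeline detects arrival and issues AIMoveTo after per-point delays, starting on BeginPlay, trigger overlap or waiting-sphere overlap.
; Tick drives look-at focus, the waiting sphere and optional target UI.
; The construction script places debug markers, trace-checks points for ground and aligns trigger actors, alongside spline-editing helper events.
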(fn `UserConstructionScript`
  (bind _spline (`self.Spline`))
  (bind _spline_2 (`self.Spline`))
  (bind _spline_3 (`self.Spline`))
  (bind _trigger_box_ (`self.Trigger Box `))
  (bind _spline_4 (`self.Spline`))
  ;[1 0 0.05951] Construction Script
  (`/Engine/EditorBlueprintResources/StandardMacros.IsValid` (`self.Character Reference`)
    (:`Is Valid`
      (`|ExecutionSequence`
        (:`then_0`
          (`|ExecutionSequence`
            (:`then_0`
              ;;[1 0 0.05951] Set Actor Location
              (`self.K2_SetActorLocation` (`self.K2_GetActorLocation` (`self.Character Reference`))))
            (:`then_1`
              ;;[1 0 0.05951] Add Point index in Array
              (for _index (range 1 (+ (`SplineComponent.GetNumberOfSplinePoints` (`self.Spline`)) 1))
                (`KismetArrayLibrary.Array_Add` (`self.Index Array`) _index)))
            (:`then_2`
              ;;[1 0 0.05951] Set Bad Point
              (for _array_element (`self.Index Array`)
                (bind _returnvalue (`SplineComponent.GetLocationAtSplinePoint` _spline _array_element "World"))
                (bind _returnvalue_2 (+ (* (`SceneComponent.GetUpVector` _spline) -120.0) _returnvalue))
                (bind (_outhit _returnvalue_3) (`KismetSystemLibrary.LineTraceSingle` _returnvalue _returnvalue_2 "TraceTypeQuery1"))
                (if _returnvalue_3
                  (`SceneComponent.SetVisibility` (stale _returnvalue_4) true false)
                  (else
                    (bind _returnvalue_4 (`AddComponent|NODE_AddBillboardComponent-0` :`bManualAttachment` true :`RelativeTransform` (`KismetMathLibrary.MakeTransform` _returnvalue_2)))))))
            (:`then_3`
              ;;[1 0 0.05951] Spawn Waiting Sphere Collision
              (if (`self.Waiting`)
                (bind _returnvalue_5 (`AddComponent|NODE_AddSphereComponent-1`))
                (bind _output_get (set `self.WaitingCollision` _returnvalue_5))
                (`SphereComponent.SetSphereRadius` _output_get (`self.Waiting Sphere Radius`) true)))))
        (:`then_1`
          ;;[1 0 0.05951] End Point Debug
          (`SceneComponent.K2_SetWorldLocation` (`self.End Point`) (+ (`SplineComponent.GetLocationAtSplinePoint` _spline_2 (`SplineComponent.GetNumberOfSplinePoints` _spline_2) "World") (* (`SceneComponent.GetUpVector` _spline_2) 150.0)) false false)
          ;;[1 0 0.05951] Start Point Debug
          (`SceneComponent.K2_SetWorldLocation` (`self.Start Point`) (+ (`SplineComponent.GetLocationAtSplinePoint` _spline_3 0 "World") (* (`SceneComponent.GetUpVector` _spline_3) 150.0)) false false))
        (:`then_2`
          ;;[1 0 0.05951] Start Movement With Trigger / Debug
          (if (`|EnumEquality` (`self.Start Movement With`) "NewEnumerator1")
            (`SceneComponent.K2_SetWorldLocation` _trigger_box_ (+ (`self.K2_GetActorLocation` (`self.Box Trigger Begin Overlap`)) (* (`SceneComponent.GetUpVector` (`self.Spline`)) 150.0)) false false)
            (`SceneComponent.SetVisibility` _trigger_box_ true false)
            (else
              (`SceneComponent.SetVisibility` _trigger_box_ false false))))
        (:`then_3`
          ;;[1 0 0.05951] Overlap Trigger Box Logic
          (for _array_element_2 (`self.Overlap Actor`)
            (bind (_overlaptrigger _jumpindex _originlocation _originrotation _scale) (break `/Game/SplineWaypointSystemV1/Blueprint/Structure/BP_OverlapStructure` _array_element_2))
            (`/Engine/EditorBlueprintResources/StandardMacros.IsValid` _overlaptrigger
              (:`Is Valid`
                (if (> _jumpindex 0)
                  (`self.K2_SetActorLocation` _overlaptrigger (+ _originlocation (`SplineComponent.GetLocationAtSplinePoint` _spline_4 _jumpindex "World")) false false)
                  (`self.K2_SetActorRotation` _overlaptrigger (`KismetMathLibrary.NormalizedDeltaRotator` (`SplineComponent.GetRotationAtSplinePoint` _spline_4 (- _jumpindex 1) "World") _originrotation) false)
                  (`self.SetActorRelativeScale3D` _overlaptrigger _scale)
                  (bind _returnvalue_6 (`AddComponent|NODE_AddBillboardComponent-1` :`bManualAttachment` true :`RelativeTransform` (`KismetMathLibrary.MakeTransform` (+ (`self.K2_GetActorLocation` _overlaptrigger) (* (`SceneComponent.GetUpVector` (`self.Spline`)) 150.0)))))
                  (`SceneComponent.SetVisibility` _returnvalue_6 true false))))))))))