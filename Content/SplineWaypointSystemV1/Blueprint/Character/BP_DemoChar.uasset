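; BP_DemoChar is the demo player character for the SplineWaypointSystemV1 content.
; MoveForward and MoveRight axes feed AddMovementInput along directions built from control yaw only, keeping movement horizontal regardless of camera pitch.
; Mouse X drives controller yaw and Mouse Y drives inverted controller pitch.
; The construction script is empty.
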(event `InputAxis|MoveRight`
  (params (AxisValue :type "Float (single-precision)"))
  ;[1 0 0.05951] Movement
  (`self.AddMovementInput` (`KismetMathLibrary.GetRightVector` (`KismetMathLibrary.MakeRotator` 0.0 0.0 (.yaw (`self.GetControlRotation`)))) AxisValue))

(event `InputAxis|MoveForward`
  (params (AxisValue :type "Float (single-precision)"))
  ;[1 0 0.05951] Movement
  (`self.AddMovementInput` (`KismetMathLibrary.GetForwardVector` (`KismetMathLibrary.MakeRotator` 0.0 0.0 (.yaw (`self.GetControlRotation`)))) AxisValue))

(event `InputAxisKey|MouseX`
  (params (AxisValue :type "Float (single-precision)"))
  ;[1 0 0.05951] Mouse
  (`self.AddControllerYawInput` AxisValue))

(event `InputAxisKey|MouseY`
  (params (AxisValue :type "Float (single-precision)"))
  ;[1 0 0.05951] Mouse
  (`self.AddControllerPitchInput` (* AxisValue -1.0)))

(fn `UserConstructionScript`)