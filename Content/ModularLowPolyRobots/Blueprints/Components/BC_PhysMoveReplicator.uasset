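; Actor component that replicates a physics-simulated primitive's movement from server to clients, optionally auto-starting on a simulating root component.
; While ticking, the server writes transform and velocities into RepData.
; Clients apply them in OnRep, blending location by error distance within an inaccuracy threshold to soften small corrections.
; Optional wake/sleep bindings switch the owner's net update frequency and component tick to save bandwidth at rest.
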(event `self.ReceiveBeginPlay`
  ;[1 1 1] get data
  (set `self.OwnerActor` (`self.GetOwner`))
  (set `self.Authority` (`Actor.HasAuthority` (`self.OwnerActor`)))
  ;[1 1 1] autostart
  (if (`self.AutoStart`)
    (bind _asprimitive_component (cast `PrimitiveComponent` (`Actor.RootComponent` (`self.OwnerActor`))))
    (if (`SceneComponent.IsSimulatingPhysics` _asprimitive_component "None")
      (`self.SetSyncComponent` _asprimitive_component true))))

(event `SimulationWake`
  (params (WakingComponent :type "PrimitiveComponent Object Reference") (BoneName :type Name))
  ;[1 1 1] Net update frequency changing
  (if (`self.Authority`)
    (set `Actor.NetUpdateFrequency` (`self.WakeUpdateFrequency`) (`self.OwnerActor`))
    (set `Actor.MinNetUpdateFrequency` (* (`self.WakeUpdateFrequency`) (`self.MinUpdateMultiplier`)) (`self.OwnerActor`))
    (`Actor.ForceNetUpdate` (`self.OwnerActor`))
    (`self.SetComponentTickEnabled` true)))

(event `self.ReceiveTick`
  (params (DeltaSeconds :type "Float (single-precision)"))
  (bind (_returnvalue_location _returnvalue_rotation) (`KismetMathLibrary.BreakTransform` (`SceneComponent.K2_GetComponentToWorld` (`self.PhysComponent`))))
  ;[1 1 1] send data
  (if (`self.Authority`)
    (set `self.RepData` (make `/Game/ModularLowPolyRobots/Blueprints/Components/S_MoveReplicationData` _returnvalue_location _returnvalue_rotation (`SceneComponent.GetComponentVelocity` (`self.PhysComponent`)) (`PrimitiveComponent.GetPhysicsAngularVelocityInDegrees` (`self.PhysComponent`) "None")))))

(event `SimulationSleep`
  (params (SleepingComponent :type "PrimitiveComponent Object Reference") (BoneName :type Name))
  ;[1 1 1] Net update frequency changing
  (if (`self.Authority`)
    (set `Actor.NetUpdateFrequency` (`self.SleepUpdateFrequency`) (`self.OwnerActor`))
    (set `Actor.MinNetUpdateFrequency` (* (`self.SleepUpdateFrequency`) (`self.MinUpdateMultiplier`)) (`self.OwnerActor`))
    (`self.SetComponentTickEnabled` false)))

(fn `OnRep_RepData`
  (locals (RepLocation :type "Vector Structure" :default (0.0 0.0 0.0)))
  (bind (_repdata_location _repdata_rotation) (break `/Game/ModularLowPolyRobots/Blueprints/Components/S_MoveReplicationData` (`self.RepData`)))
  (bind _repdata_location_2 (break `/Game/ModularLowPolyRobots/Blueprints/Components/S_MoveReplicationData` (`self.RepData`)))
  (bind _repdata_location_3 (break `/Game/ModularLowPolyRobots/Blueprints/Components/S_MoveReplicationData` (`self.RepData`)))
  (bind _repdata_location_4 (break `/Game/ModularLowPolyRobots/Blueprints/Components/S_MoveReplicationData` (`self.RepData`)))
  (bind (_repdata_location_5 _repdata_rotation_2 _repdata_linearvelocity) (break `/Game/ModularLowPolyRobots/Blueprints/Components/S_MoveReplicationData` (`self.RepData`)))
  (bind (_repdata_location_6 _repdata_rotation_3 _repdata_linearvelocity_2 _repdata_angularvelocity) (break `/Game/ModularLowPolyRobots/Blueprints/Components/S_MoveReplicationData` (`self.RepData`)))
  (bind _returnvalue (`SceneComponent.K2_GetComponentLocation` (`self.PhysComponent`)))
  (if (not (`self.Authority`))
    (`/Engine/EditorBlueprintResources/StandardMacros.IsValid` (`self.PhysComponent`)
      (:`Is Valid`
        ;[1 1 1] set velocity
        (`PrimitiveComponent.SetPhysicsLinearVelocity` (`self.PhysComponent`) _repdata_linearvelocity false "None")
        (`PrimitiveComponent.SetPhysicsAngularVelocityInDegrees` (`self.PhysComponent`) _repdata_angularvelocity false "None")
        (`|ExecutionSequence`
          (:`then_0`
            ;[1 1 1] get new location
            (if (== (`self.SetLocationInaccuaracy`) 0.0)
              (set `local.RepLocation` _repdata_location_3)
              (else
                (set `local.RepLocation` (`KismetMathLibrary.VLerp` _returnvalue _repdata_location_2 (/ (`KismetMathLibrary.FClamp` (`KismetMathLibrary.VSize` (- _returnvalue _repdata_location_4)) 0.0 (`self.SetLocationInaccuaracy`)) (`self.SetLocationInaccuaracy`)))))))
          (:`then_1`
            ;[1 1 1] set loc rot
            (`SceneComponent.K2_SetWorldLocationAndRotation` (`self.PhysComponent`) (`local.RepLocation`) _repdata_rotation false true)))))))

(fn `SetSyncComponent`
  (params (SimulatedComponent :type "PrimitiveComponent Object Reference") (SetActivate :type Boolean))
  (set `self.PhysComponent` SimulatedComponent)
  (`|ExecutionSequence`
    (:`then_0`
      ;[1 1 1] enable tick on server
      (if (`local.SetActivate`)
        (if (`self.Authority`)
          (`self.SetComponentTickEnabled` true))))
    (:`then_1`
      ;[1 1 1] bind to sleep and wake events
      (if (`self.AllowSyncFrequencyChanging`)
        (add `PrimitiveComponent.OnComponentWake` (`self.PhysComponent`) (`|CreateDelegate` :!event `SimulationWake`))
        (add `PrimitiveComponent.OnComponentSleep` (`self.PhysComponent`) (`|CreateDelegate` :!event `SimulationSleep`))))))