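; Game mode that gives each joining player an unoccupied PlayerStart in the modular low-poly robots project.
; ChoosePlayerStart claims the first start tagged None, tags it Used and records it in a map keyed by controller, falling back to a random start when all are taken.
; It also binds to the controller's destroyed event, which resets that start's tag and removes the map entry when the player leaves.
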(event `PlayerLeft`
  (params (DestroyedActor :type "Actor Object Reference"))
  ;[1 1 1] clear used tag in player start actor when a player laft
  (bind _ascontroller (cast `Controller` DestroyedActor))
  (set `PlayerStart.PlayerStartTag` "None" (`BlueprintMapLibrary.Map_Find` (`self.PlayerStartPoints`) _ascontroller))
  (`BlueprintMapLibrary.Map_Remove` (`self.PlayerStartPoints`) _ascontroller))

(fn `ChoosePlayerStart`
  (params (Player :type "Controller Object Reference"))
  (returns (ReturnValue :type "Actor Object Reference"))
  (locals (CurrentPlayerStart :type "PlayerStart Object Reference"))
  (add `self.OnDestroyed` (`local.Player`) (`|CreateDelegate` :!event `PlayerLeft`))
  (bind _outactors (`GameplayStatics.GetAllActorsOfClass` "/Script/Engine.PlayerStart"))
  (for _array_element _outactors
    (bind _output_get (set `local.CurrentPlayerStart` _array_element))
    (if (== (`PlayerStart.PlayerStartTag` _output_get) "None")
      (set `PlayerStart.PlayerStartTag` "Used" (`local.CurrentPlayerStart`))
      (`BlueprintMapLibrary.Map_Add` (`self.PlayerStartPoints`) (`local.Player`) (`local.CurrentPlayerStart`))
      (return (`local.CurrentPlayerStart`))))
  (return (`|GetArrayItem` _outactors (`KismetMathLibrary.RandomInteger` (`KismetArrayLibrary.Array_LastIndex` _outactors)))))

(fn `UserConstructionScript`)