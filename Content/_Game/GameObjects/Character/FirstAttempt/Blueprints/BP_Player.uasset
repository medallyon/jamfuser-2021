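; Player character for the robber, with a cursor-aimed mesh, walk and sprint speeds, a velocity-burst dash and a HUD.
; Thumb mouse buttons rotate the spring arm in 90-degree steps, feeding a yaw offset into movement input.
; Tick updates facing, sets ABP_Robber's Moving flag and handles hiding, which conceals the mesh and halts movement.
; ChangeCamera can reposition the camera to a home-base point; click-to-move logic is left disconnected.
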(event `self.ReceiveBeginPlay`
  (`|ExecutionSequence`
    (:`then_0`
      (bind _returnvalue (`|CreateWidget` "/Game/_Game/GameObjects/Character/HUD.HUD_C"))
      (`UserWidget.AddToViewport` _returnvalue 0))
    (:`then_1`
      ;[0 0.25 1] Set Initial Vars
      (set `PlayerController.bShowMouseCursor` true (`GameplayStatics.GetPlayerController` 0))
      (set `self.Camera Location` (`SceneComponent.RelativeLocation` (`self.Camera`)))
      (set `self.Camera Rotation` (`SceneComponent.RelativeRotation` (`self.Camera`))))))

(event `InputAction|Interact`
  (params (Key :type "Key Structure"))
  (:`Pressed`
    (set `self.Interact` true))
  (:`Released`
    (set `self.Interact` false)))

(event `Key|SpaceBar`
  (params (Key :type "Key Structure"))
  (bind _charactermovement (`self.CharacterMovement`))
  (:`Pressed`
    (if (not (`self.Dash`))
      (set `self.Dash` true)
      (set `MovementComponent.Velocity` (* (`MovementComponent.Velocity` _charactermovement) 15) _charactermovement)
      (`KismetSystemLibrary.Delay` 0.2)
      (set `self.Dash` false))))

(event `Key|ThumbMouseButton`
  (params (Key :type "Key Structure"))
  (bind _springarm (`self.SpringArm`))
  (bind (_returnvalue_roll _returnvalue_pitch _returnvalue_yaw) (`KismetMathLibrary.BreakRotator` (`SpringArmComponent.GetTargetRotation` _springarm)))
  (:`Pressed`
    (`SceneComponent.K2_SetWorldRotation` _springarm (`KismetMathLibrary.MakeRotator` 0.0 0.0 (+ _returnvalue_yaw 90.0)) false false)
    (set `self.Rotation` (+ (`self.Rotation`) 90.0))))

(event `Key|ThumbMouseButton2`
  (params (Key :type "Key Structure"))
  (bind _springarm (`self.SpringArm`))
  (bind (_returnvalue_roll _returnvalue_pitch _returnvalue_yaw) (`KismetMathLibrary.BreakRotator` (`SpringArmComponent.GetTargetRotation` _springarm)))
  (:`Pressed`
    (`SceneComponent.K2_SetWorldRotation` _springarm (`KismetMathLibrary.MakeRotator` 0.0 0.0 (+ _returnvalue_yaw -90.0)) false false)
    (set `self.Rotation` (+ (`self.Rotation`) -90.0))))

(event `InputAxis|MoveForward/Backwards`
  (params (AxisValue :type "Float (single-precision)"))
  ;[1 0.5156 0] Move Player
  (`self.AddMovementInput` (`KismetMathLibrary.GetForwardVector` (`KismetMathLibrary.MakeRotator` 0.0 0.0 (+ (.yaw (`self.GetControlRotation`)) (`self.Rotation`)))) AxisValue))

(event `InputAxis|MoveRight/Left`
  (params (AxisValue :type "Float (single-precision)"))
  ;[1 0.5156 0] Move Player
  (`self.AddMovementInput` (`KismetMathLibrary.GetRightVector` (`KismetMathLibrary.MakeRotator` 0.0 0.0 (+ (.yaw (`self.GetControlRotation`)) (`self.Rotation`)))) AxisValue))

(event `InputAction|SprintAction`
  (params (Key :type "Key Structure"))
  (bind _charactermovement (`self.CharacterMovement`))
  ;[0 1 0.3438] Move Type
  (:`Pressed`
    (set `CharacterMovementComponent.MaxWalkSpeed` 1000.0 _charactermovement))
  (:`Released`
    (set `CharacterMovementComponent.MaxWalkSpeed` 600.0 _charactermovement)))

(event `self.ReceiveTick`
  (params (DeltaSeconds :type "Float (single-precision)"))
  ;[1 0 0.8203] Tick
  (`|ExecutionSequence`
    (:`then_0`
      (`self.RotateCharacter`))
    (:`then_1`
      (`self.Moving?`))
    (:`then_2`
      (`self.Hidden`))))

(event `Key|RightMouseButton`
  (params (Key :type "Key Structure"))
  ;[0 0.03906 1] Check Mouse Down
  (:`Pressed`
    (set `self.Is Mouse Down?` true))
  (:`Released`
    (set `self.Is Mouse Down?` false)))

(event `InputAction|WalkAction`
  (params (Key :type "Key Structure"))
  (bind _charactermovement (`self.CharacterMovement`))
  ;[0 1 0.3438] Move Type
  (:`Pressed`
    (set `CharacterMovementComponent.MaxWalkSpeed` 300.0 _charactermovement))
  (:`Released`
    (set `CharacterMovementComponent.MaxWalkSpeed` 600.0 _charactermovement)))

(event `GainedLoot`
  (params (NewParam :type Integer)))

(event `Stop Moving`)

(fn `Change Camera`
  (if (not (== (`SceneComponent.K2_GetComponentRotation` (`self.Camera`)) (struct) :`ErrorTolerance` 0.1))
    (bind _returnvalue (`GameplayStatics.GetActorOfClass` "/Game/_Game/GameObjects/HomeBase/Blueprints/BP_HomeBaseCombined_Blocking.BP_HomeBaseCombined_Blocking_C"))
    (`SceneComponent.K2_SetWorldLocationAndRotation` :`self` (`self.Camera`) :`NewLocation` (`SceneComponent.K2_GetComponentLocation` (`/Game/_Game/GameObjects/HomeBase/Blueprints/BP_HomeBaseCombined_Blocking.Camera Pointing On Screen` _returnvalue)))
    (else
      (`SceneComponent.K2_SetRelativeLocationAndRotation` (`self.Camera`) (`self.Camera Location`) (`self.Camera Rotation`) false false))))

(fn `Hidden`
  (bind _mesh (`self.Mesh`))
  (if (`self.Hiding`)
    (`SceneComponent.SetHiddenInGame` _mesh true false)
    (`MovementComponent.StopMovementImmediately` (`self.CharacterMovement`))
    (else
      (`SceneComponent.SetHiddenInGame` _mesh false false))))

(fn `Moving?`
  (bind _returnvalue (`SkeletalMeshComponent.GetAnimInstance` (`self.Mesh`)))
  (if (== (`self.GetVelocity`) (0.0 0.0 0.0))
    (bind _asabp_robber (cast `/Game/_Game/GameObjects/Character/FirstAttempt/Blueprints/ABP_Robber` _returnvalue))
    (set `/Game/_Game/GameObjects/Character/FirstAttempt/Blueprints/ABP_Robber.Moving` false _asabp_robber)
    (else
      (bind _asabp_robber_2 (cast `/Game/_Game/GameObjects/Character/FirstAttempt/Blueprints/ABP_Robber` _returnvalue))
      (set `/Game/_Game/GameObjects/Character/FirstAttempt/Blueprints/ABP_Robber.Moving` true _asabp_robber_2)
      (set `self.Hiding` false))))

(fn `RotateCharacter`
  (bind (_returnvalue_roll _returnvalue_pitch) (`KismetMathLibrary.BreakRotator` (`self.K2_GetActorRotation`)))
  (bind (_returnvalue_roll_2 _returnvalue_pitch_2 _returnvalue_yaw) (`KismetMathLibrary.BreakRotator` (`KismetMathLibrary.FindLookAtRotation` (`self.K2_GetActorLocation`) (`.Location` (`GameplayStatics.BreakHitResult` (`PlayerController.GetHitResultUnderCursorByChannel` (`GameplayStatics.GetPlayerController` 0) "TraceTypeQuery1" true))))))
  (`SceneComponent.K2_SetWorldRotation` (`self.Mesh`) (`KismetMathLibrary.MakeRotator` _returnvalue_roll _returnvalue_pitch (+ _returnvalue_yaw -90.0)) false false))

(fn `UserConstructionScript`)