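; BP_Interaction_Area is a home base trigger zone that lets the player toggle a camera refocus with the E key.
; Player overlap sets a can-interact flag and shows an interaction hint widget, which is removed on exit.
; While the flag is set, each press calls ChangeCamera on BP_Player, and a FlipFlop alternates between disabling pawn input and stopping movement, then re-enabling input.
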(event `Key|E`
  (params (Key :type "Key Structure"))
  (bind _returnvalue (`GameplayStatics.GetPlayerPawn` 0))
  (bind _returnvalue_2 (`GameplayStatics.GetPlayerController` 0))
  ;[0.9453 1 0] ReFocus Camera
  (:`Pressed`
    (if (`self.Can Iteract?`)
      (`|ExecutionSequence`
        (:`then_0`
          (bind _returnvalue_3 (`GameplayStatics.GetActorOfClass` "/Game/_Game/GameObjects/Character/Blueprints/BP_Player.BP_Player_C"))
          (`/Game/_Game/GameObjects/Character/Blueprints/BP_Player.Change Camera` _returnvalue_3))
        (:`then_1`
          (`/Engine/EditorBlueprintResources/StandardMacros.FlipFlop`
            (:`A`
              (`self.DisableInput` _returnvalue _returnvalue_2)
              (bind _asbp_player (cast `/Game/_Game/GameObjects/Character/Blueprints/BP_Player` _returnvalue))
              (`/Game/_Game/GameObjects/Character/Blueprints/BP_Player.Stop Moving` _asbp_player))
            (:`B`
              (`self.EnableInput` _returnvalue _returnvalue_2))))))))

(event `self.ReceiveActorBeginOverlap`
  (params (OtherActor :type "Actor Object Reference"))
  ;[0 0.9062 1] Interaction Hint
  (cast `/Game/_Game/GameObjects/Character/Blueprints/BP_Player` OtherActor)
  (set `self.Can Iteract?` true)
  (bind _returnvalue (`|CreateWidget` "/Game/_Game/UI/Widgets/HUD/WBP_InteractionHint.WBP_InteractionHint_C"))
  (`UserWidget.AddToViewport` _returnvalue 0))

(event `self.ReceiveActorEndOverlap`
  (params (OtherActor :type "Actor Object Reference"))
  ;[0 0.9062 1] Interaction Hint
  (cast `/Game/_Game/GameObjects/Character/Blueprints/BP_Player` OtherActor)
  (set `self.Can Iteract?` false)
  (`Widget.RemoveFromParent` (stale `self.ReceiveActorBeginOverlap` _returnvalue)))

(fn `UserConstructionScript`)