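; BP_InteractionArea is a home base trigger that lets the player enter and leave a screen interaction with the E key.
; Player overlap enables interaction and shows a hint widget, removed when the overlap ends.
; Each press flips a FlipFlop into HandleScreenInteraction, which switches the player camera and toggles pawn input and the hint.
; It also calls Interact on HomeBase with its Number as source and the toggle state.
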(event `Key|E` :consume false
  (params (Key :type "Key Structure"))
  ;[0.9453 1 0] ReFocus Camera
  (:`Pressed`
    (if (`self.Can Iteract?`)
      (`/Engine/EditorBlueprintResources/StandardMacros.IsValid` (`self.Home Base`)
        (:`Is Valid`
          (bind _isa (`/Engine/EditorBlueprintResources/StandardMacros.FlipFlop`)
            (:`A`
              _)
            (:`B`
              _))
          (`self.Handle Screen Interaction` _isa))))))

(event `self.ReceiveActorEndOverlap`
  (params (OtherActor :type "Actor Object Reference"))
  ;[0 0.9062 1] Interaction Hint
  (castclass `/Game/_Game/GameObjects/Character/WorkingAttempt/BP_Player_Character` (`GameplayStatics.GetObjectClass` OtherActor))
  (set `self.Can Iteract?` false)
  (`/Engine/EditorBlueprintResources/StandardMacros.IsValid` (stale `self.ReceiveActorBeginOverlap` _output_get)
    (:`Is Valid`
      (`Widget.RemoveFromParent` (stale `self.ReceiveActorBeginOverlap` _output_get)))))

(event `self.ReceiveActorBeginOverlap`
  (params (OtherActor :type "Actor Object Reference"))
  ;[0 0.9062 1] Interaction Hint
  (castclass `/Game/_Game/GameObjects/Character/WorkingAttempt/BP_Player_Character` (`GameplayStatics.GetObjectClass` OtherActor))
  (set `self.Can Iteract?` true)
  (bind _returnvalue (`|CreateWidget` "/Game/_Game/UI/Widgets/HUD/WBP_InteractionHint.WBP_InteractionHint_C"))
  (bind _output_get (set `self.Interaction Widget Hint` _returnvalue))
  (`UserWidget.AddToViewport` _output_get 0))

(fn `Handle Screen Interaction`
  (params (`Is Entering Screen` :type Boolean))
  (bind _returnvalue (`GameplayStatics.GetPlayerPawn` 0))
  (bind _returnvalue_2 (`GameplayStatics.GetPlayerController` 0))
  (bind _number (`self.Number`))
  (bind _returnvalue_3 (`GameplayStatics.GetActorOfClass` "/Game/_Game/GameObjects/Character/WorkingAttempt/BP_Player_Character.BP_Player_Character_C"))
  (`/Game/_Game/GameObjects/Character/WorkingAttempt/BP_Player_Character.Change Camera` _returnvalue_3)
  (if `Is Entering Screen`
    (`self.DisableInput` _returnvalue _returnvalue_2)
    (`Widget.RemoveFromParent` (`self.Interaction Widget Hint`))
    (`/Game/_Game/GameObjects/HomeBase/Blueprints/BP_HomeBaseCombined_Working.Interact` (`self.Home Base`) _number true)
    (else
      (`self.EnableInput` _returnvalue _returnvalue_2)
      (`UserWidget.AddToViewport` (`self.Interaction Widget Hint`) 0)
      (`/Game/_Game/GameObjects/HomeBase/Blueprints/BP_HomeBaseCombined_Working.Interact` (`self.Home Base`) _number false))))

(fn `UserConstructionScript`)