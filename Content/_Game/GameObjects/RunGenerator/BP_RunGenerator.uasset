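; Run generator actor that builds a run from randomly picked room levels, streamed in as level instances at runtime.
; Starting on BeginPlay, each step gathers and destroys all BP_RoomConnector actors, then spawns a room at a randomly chosen connector transform.
; Each room's load callback triggers the next step until the room count is reached, so loading is sequential.
; Room entrance alignment logic exists but is never run.
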(event `self.ReceiveBeginPlay`
  (`self.Load Next Room`))

(event `On Level Load`
  (`|ExecutionSequence`
    (:`then_0`
      (`/Engine/EditorBlueprintResources/StandardMacros.IncrementInt` (`self.Rooms Loaded`)))
    (:`then_2`
      (clear `LevelStreaming.OnLevelLoaded` (`self.Most Recent Room`))
      (`self.Load Next Room`))))

(event `Load Next Room`
  (bind _possible_rooms_rooms (break `/Game/_Game/Maps/Runs/01/S_Rooms_Run_01` (`self.Possible Rooms`)))
  (if (< (`self.Rooms Loaded`) (`self.Number of Rooms`))
    (bind _connector_transforms (`self.Get All RoomConnector Transforms` true))
    (bind _outitem (`KismetArrayLibrary.Array_Random` _connector_transforms))
    (bind (_boutsuccess _returnvalue) (`LevelStreamingDynamic.LoadLevelInstance` (`KismetArrayLibrary.Array_Random` _possible_rooms_rooms) (.location _outitem) (.rotation _outitem)))
    (bind _output_get (set `self.Most Recent Room` _returnvalue))
    (add `LevelStreaming.OnLevelLoaded` _output_get (delegate `On Level Load`))))

(fn `Get All RoomConnector Transforms`
  (params (`Destroy Actors?` :type Boolean))
  (returns (`Connector Transforms` :type "Array of Transform Structure"))
  (locals (Transforms :type "Array of Transform Structure"))
  (bind _outactors (`GameplayStatics.GetAllActorsOfClass` "/Game/_Game/GameObjects/RoomConnector/BP_RoomConnector.BP_RoomConnector_C"))
  (bind (_arrayindex _arrayelement) (`/Engine/EditorBlueprintResources/StandardMacros.ReverseForEachLoop` _outactors)
    (:`LoopBody`
      (`|ExecutionSequence`
        (:`then_0`
          (`KismetArrayLibrary.Array_AddUnique` (`local.Transforms`) (`self.GetTransform` _arrayelement)))
        (:`then_1`
          (if (`local.Destroy Actors?`)
            (`self.K2_DestroyActor` _arrayelement)))))
    (:`Completed`
      (return (`local.Transforms`)))))

(fn `Get All RoomEntrance Transforms`
  (params (`Destroy Actors?` :type Boolean))
  (returns (`Entrance Transforms` :type "Array of Transform Structure"))
  (locals (Transforms :type "Array of Transform Structure"))
  (bind _outactors (`GameplayStatics.GetAllActorsOfClass` "/Game/_Game/GameObjects/RoomConnector/BP_RoomEntrance.BP_RoomEntrance_C"))
  (bind (_arrayindex _arrayelement) (`/Engine/EditorBlueprintResources/StandardMacros.ReverseForEachLoop` _outactors)
    (:`LoopBody`
      (`|ExecutionSequence`
        (:`then_0`
          (`KismetArrayLibrary.Array_AddUnique` (`local.Transforms`) (`self.GetTransform` _arrayelement)))
        (:`then_1`
          (if (`local.Destroy Actors?`)
            (`self.K2_DestroyActor` _arrayelement)))))
    (:`Completed`
      (return (`local.Transforms`)))))

(fn `UserConstructionScript`)