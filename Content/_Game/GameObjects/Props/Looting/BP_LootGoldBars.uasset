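; Lootable gold bar prop that grants the player 100 Loot when taken, then destroys itself.
; BeginPlay is set up to pick Stack or Plate at random, but RandomInteger(1) always returns 0, so Plate is shown.
; Box overlap shows a widget and polls Interact through Delay loops, filling the character's Unlock while held and resetting it otherwise.
; Full Unlock activates StaticMeshComponent, whose activation event handles the pickup.
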(event `self.ReceiveBeginPlay`
  (bind _returnvalue (`KismetMathLibrary.RandomInteger` 1))
  (bind _stack (`self.Stack`))
  (bind _plate (`self.Plate`))
  (`|ExecutionSequence`
    (:`then_0`
      (if (== _returnvalue 0)
        (`SceneComponent.SetVisibility` _stack false true)
        (`SceneComponent.SetVisibility` _plate true true)))
    (:`then_1`
      (if (== _returnvalue 1)
        (`SceneComponent.SetVisibility` _plate false true)
        (`SceneComponent.SetVisibility` _stack true true)))
    (:`then_2`
      (`SceneComponent.SetVisibility` (`self.Widget`) false false))))

(event `self.Box.OnComponentBeginOverlap`
  (params (OverlappedComponent :type "PrimitiveComponent Object Reference") (OtherActor :type "Actor Object Reference") (OtherComp :type "PrimitiveComponent Object Reference") (OtherBodyIndex :type Integer) (bFromSweep :type Boolean) (SweepResult :type "HitResult Structure (by ref)"))
  (bind _asbp_player (cast `` OtherActor))
  (set `/Game/_Game/GameObjects/Props/Looting/BP_LootGoldBars.Unlock` 0.0 _asbp_player)
  (set `self.Overlapped` true)
  (if (`self.Overlapped`) :!label _label
    (bind _asbp_player_2 (cast `` OtherActor))
    (`SceneComponent.SetVisibility` (`self.Widget`) true false)
    (if (`/Game/_Game/GameObjects/Props/Looting/BP_LootGoldBars.Interact` _asbp_player_2) :!label _label_2
      (bind _unlock (`/Game/_Game/GameObjects/Props/Looting/BP_LootGoldBars.Unlock` _asbp_player_2))
      (if (>= _unlock 1.0)
        (`ActorComponent.Activate` (`self.StaticMeshComponent`) false)
        (else
          (set `/Game/_Game/GameObjects/Props/Looting/BP_LootGoldBars.Unlock` (+ _unlock 0.25) _asbp_player_2)
          (`KismetSystemLibrary.Delay` 0.1)
          (goto _label_2)))
      (else
        (`KismetSystemLibrary.Delay` 0.05)
        (set `/Game/_Game/GameObjects/Props/Looting/BP_LootGoldBars.Unlock` 0.0 _asbp_player_2)
        (goto _label)))))

(event `self.Box.OnComponentEndOverlap`
  (params (OverlappedComponent :type "PrimitiveComponent Object Reference") (OtherActor :type "Actor Object Reference") (OtherComp :type "PrimitiveComponent Object Reference") (OtherBodyIndex :type Integer))
  (set `self.Overlapped` false)
  (`SceneComponent.SetVisibility` (`self.Widget`) false false))

(event `self.StaticMeshComponent.OnComponentActivated`
  (params (Component :type "ActorComponent Object Reference") (bReset :type Boolean))
  (`SceneComponent.SetVisibility` (`self.Stack`) false true)
  (`SceneComponent.SetVisibility` (`self.Plate`) false true)
  (`PrimitiveComponent.SetCollisionEnabled` (`self.Box`) "NoCollision")
  (bind _asbp_player (cast `` (`GameplayStatics.GetPlayerCharacter` 0)))
  (set `/Game/_Game/GameObjects/Props/Looting/BP_LootGoldBars.Loot` (+ (`/Game/_Game/GameObjects/Props/Looting/BP_LootGoldBars.Loot` _asbp_player) 100) _asbp_player)
  (`self.K2_DestroyActor`))

(fn `UserConstructionScript`)