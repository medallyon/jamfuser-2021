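; Lootable small jewelry prop that randomizes its look on BeginPlay among rings, bracelets and two necklaces, using a separate random roll per variant.
; Overlapping the box shows a widget and starts a delay-based polling loop that fills the actor's Unlock while Interact is held, resetting it otherwise.
; At full Unlock, activating the static mesh component acts as the collection trigger, hiding everything, disabling box collision and adding Loot to the player.
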(event `self.ReceiveBeginPlay`
  (bind _returnvalue (`KismetMathLibrary.RandomInteger` 4))
  (bind _necklace_black (`self.Necklace Black`))
  (bind _necklace_white (`self.Necklace White`))
  (`|ExecutionSequence`
    (:`then_0`
      (if (== _returnvalue 0)
        (`SceneComponent.SetVisibility` _necklace_black false true)
        (`SceneComponent.SetVisibility` _necklace_white false true)
        (`SceneComponent.SetVisibility` (`self.Bracelets`) false true)
        (`SceneComponent.SetVisibility` (`self.Rings`) true true)))
    (:`then_1`
      (if (== _returnvalue 1)
        (`SceneComponent.SetVisibility` _necklace_black false true)
        (`SceneComponent.SetVisibility` _necklace_white false true)
        (`SceneComponent.SetVisibility` (`self.Rings`) false true)
        (`SceneComponent.SetVisibility` (`self.Bracelets`) true true)))
    (:`then_2`
      (if (== _returnvalue 2)
        (`SceneComponent.SetVisibility` _necklace_black false true)
        (`SceneComponent.SetVisibility` (`self.Bracelets`) false true)
        (`SceneComponent.SetVisibility` (`self.Rings`) false true)
        (`SceneComponent.SetVisibility` _necklace_white true true)))
    (:`then_3`
      (if (== _returnvalue 3)
        (`SceneComponent.SetVisibility` _necklace_white false true)
        (`SceneComponent.SetVisibility` (`self.Bracelets`) false true)
        (`SceneComponent.SetVisibility` (`self.Rings`) false true)
        (`SceneComponent.SetVisibility` _necklace_black true true)))
    (:`then_4`
      (`SceneComponent.SetVisibility` (`self.Widget`) false false))))

(event `self.Box.OnComponentBeginOverlap`
  (params (OverlappedComponent :type "PrimitiveComponent Object Reference") (OtherActor :type "Actor Object Reference") (OtherComp :type "PrimitiveComponent Object Reference") (OtherBodyIndex :type Integer) (bFromSweep :type Boolean) (SweepResult :type "HitResult Structure (by ref)"))
  (bind _asbp_player (cast `` OtherActor))
  (set `/Game/_Game/GameObjects/Props/Looting/BP_LootSmallJewelery.Unlock` 0.0 _asbp_player)
  (set `self.Overlapped` true)
  (if (`self.Overlapped`) :!label _label
    (bind _asbp_player_2 (cast `` OtherActor))
    (`SceneComponent.SetVisibility` (`self.Widget`) true false)
    (if (`/Game/_Game/GameObjects/Props/Looting/BP_LootSmallJewelery.Interact` _asbp_player_2) :!label _label_2
      (bind _unlock (`/Game/_Game/GameObjects/Props/Looting/BP_LootSmallJewelery.Unlock` _asbp_player_2))
      (if (>= _unlock 1.0)
        (`ActorComponent.Activate` (`self.StaticMeshComponent`) false)
        (else
          (set `/Game/_Game/GameObjects/Props/Looting/BP_LootSmallJewelery.Unlock` (+ _unlock 0.1) _asbp_player_2)
          (`KismetSystemLibrary.Delay` 0.1)
          (goto _label_2)))
      (else
        (`KismetSystemLibrary.Delay` 0.05)
        (set `/Game/_Game/GameObjects/Props/Looting/BP_LootSmallJewelery.Unlock` 0.0 _asbp_player_2)
        (goto _label)))))

(event `self.Box.OnComponentEndOverlap`
  (params (OverlappedComponent :type "PrimitiveComponent Object Reference") (OtherActor :type "Actor Object Reference") (OtherComp :type "PrimitiveComponent Object Reference") (OtherBodyIndex :type Integer))
  (set `self.Overlapped` false)
  (`SceneComponent.SetVisibility` (`self.Widget`) false false))

(event `self.StaticMeshComponent.OnComponentActivated`
  (params (Component :type "ActorComponent Object Reference") (bReset :type Boolean))
  (`SceneComponent.SetVisibility` (`self.Widget`) false true)
  (`SceneComponent.SetVisibility` (`self.Necklace Black`) false true)
  (`SceneComponent.SetVisibility` (`self.Necklace White`) false true)
  (`SceneComponent.SetVisibility` (`self.Bracelets`) false true)
  (`SceneComponent.SetVisibility` (`self.Rings`) false true)
  (`PrimitiveComponent.SetCollisionEnabled` (`self.Box`) "NoCollision")
  (bind _asbp_player (cast `` (`GameplayStatics.GetPlayerCharacter` 0)))
  (set `/Game/_Game/GameObjects/Props/Looting/BP_LootSmallJewelery.Loot` (+ (`/Game/_Game/GameObjects/Props/Looting/BP_LootSmallJewelery.Loot` _asbp_player) 150) _asbp_player))

(fn `UserConstructionScript`)