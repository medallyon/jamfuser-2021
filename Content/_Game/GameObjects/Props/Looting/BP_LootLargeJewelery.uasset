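; BP_LootLargeJewelery is a lootable jewelry prop that the player collects by holding interact inside its box trigger.
; Overlap shows the widget and runs a Delay-based polling loop that fills the character's Unlock value, resetting it when interact is released.
; A full Unlock activates the StaticMeshComponent, whose activation event hides the widget, necklace and bracelets, disables box collision and adds to the player's Loot.
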(event `self.ReceiveBeginPlay`
  (`SceneComponent.SetVisibility` (`self.Widget`) false false))

(event `self.Box.OnComponentBeginOverlap`
  (params (OverlappedComponent :type "PrimitiveComponent Object Reference") (OtherActor :type "Actor Object Reference") (OtherComp :type "PrimitiveComponent Object Reference") (OtherBodyIndex :type Integer) (bFromSweep :type Boolean) (SweepResult :type "HitResult Structure (by ref)"))
  (bind _asbp_player (cast `` OtherActor))
  (set `/Game/_Game/GameObjects/Props/Looting/BP_LootLargeJewelery.Unlock` 0.0 _asbp_player)
  (set `self.Overlapped` true)
  (if (`self.Overlapped`) :!label _label
    (bind _asbp_player_2 (cast `` OtherActor))
    (`SceneComponent.SetVisibility` (`self.Widget`) true false)
    (if (`/Game/_Game/GameObjects/Props/Looting/BP_LootLargeJewelery.Interact` _asbp_player_2) :!label _label_2
      (bind _unlock (`/Game/_Game/GameObjects/Props/Looting/BP_LootLargeJewelery.Unlock` _asbp_player_2))
      (if (>= _unlock 1.0)
        (`ActorComponent.Activate` (`self.StaticMeshComponent`) false)
        (else
          (set `/Game/_Game/GameObjects/Props/Looting/BP_LootLargeJewelery.Unlock` (+ _unlock 0.1) _asbp_player_2)
          (`KismetSystemLibrary.Delay` 0.1)
          (goto _label_2)))
      (else
        (`KismetSystemLibrary.Delay` 0.05)
        (set `/Game/_Game/GameObjects/Props/Looting/BP_LootLargeJewelery.Unlock` 0.0 _asbp_player_2)
        (goto _label)))))

(event `self.Box.OnComponentEndOverlap`
  (params (OverlappedComponent :type "PrimitiveComponent Object Reference") (OtherActor :type "Actor Object Reference") (OtherComp :type "PrimitiveComponent Object Reference") (OtherBodyIndex :type Integer))
  (set `self.Overlapped` false)
  (`SceneComponent.SetVisibility` (`self.Widget`) false false))

(event `self.StaticMeshComponent.OnComponentActivated`
  (params (Component :type "ActorComponent Object Reference") (bReset :type Boolean))
  (`SceneComponent.SetVisibility` (`self.Widget`) false true)
  (`SceneComponent.SetVisibility` (`self.Necklace`) false true)
  (`SceneComponent.SetVisibility` (`self.Bracelets`) false true)
  (`PrimitiveComponent.SetCollisionEnabled` (`self.Box`) "NoCollision")
  (bind _asbp_player (cast `` (`GameplayStatics.GetPlayerCharacter` 0)))
  (set `/Game/_Game/GameObjects/Props/Looting/BP_LootLargeJewelery.Loot` (+ (`/Game/_Game/GameObjects/Props/Looting/BP_LootLargeJewelery.Loot` _asbp_player) 250) _asbp_player))

(fn `UserConstructionScript`)