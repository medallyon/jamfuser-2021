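; Base ranged weapon item that fires a hitscan shot on left mouse press while its stats mark it as equipped.
; Fire box-traces on the Visibility channel from the Nozzle along its up vector out to the stat range, with one-frame debug drawing.
; A hit BPA_BaseEnemy receives the stat damage through its Hit function.
; SetBaseStats fills the Stats struct with hard-coded defaults and the given equipped state.
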(event `Key|LeftMouseButton`
  (params (Key :type "Key Structure"))
  (:`Pressed`
    (if (`.IsEquipped?_22_A6061ACD41B6029BBB815683C1C1258F` (break `/Game/_Game/GameObjects/Weapons/SRT_Weapon` (`self.Stats`)))
      (`self.Fire`))))

(fn `Fire`
  (bind _nozzle (`self.Nozzle`))
  (bind _returnvalue (`SceneComponent.K2_GetComponentLocation` _nozzle))
  (bind _outhit (`KismetSystemLibrary.BoxTraceSingle` :`Start` _returnvalue :`End` (+ _returnvalue (* (`KismetMathLibrary.GetUpVector` (`SceneComponent.K2_GetComponentRotation` _nozzle)) (`.Range_7_ADFE3A0348974133F742FD8A6574BFD3` (break `/Game/_Game/GameObjects/Weapons/SRT_Weapon` (`self.Stats`))))) :`HalfSize` (5.0 5.0 5.0) :`TraceChannel` "TraceTypeQuery1" :`DrawDebugType` "ForOneFrame"))
  (bind _asbpa_base_enemy (cast `/Game/_Game/GameObjects/Enemies/Dummy/BPA_BaseEnemy` (`.HitActor` (`GameplayStatics.BreakHitResult` _outhit))))
  (`/Game/_Game/GameObjects/Enemies/Dummy/BP_TargetDummy.Hit` _asbpa_base_enemy (`.Damage_8_183C89F74114DFF6259EAEACAF91E0C2` (break `/Game/_Game/GameObjects/Weapons/SRT_Weapon` (`self.Stats`)))))

(fn `Set Base Stats`
  (params (Equipped :type Boolean))
  (set `self.Stats` (make `/Game/_Game/GameObjects/Weapons/SRT_Weapon` 2000.0 5 24 0.0 0.0 Equipped)))

(fn `UserConstructionScript`)