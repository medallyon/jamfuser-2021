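; Base ranged weapon item that fires automatically while the left mouse button is held, if equipped and ammo remains.
; A delayed loop runs Fire from the current ammo count to the Stats limit, spacing shots by 1/RPM seconds, so RPM acts as shots per second.
; Each shot increments AmmoUse and box-traces forward using Range and Area, damaging any BPA_BaseEnemy hit.
; SetBaseStats fills default stats and resets the ammo counter.
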(event `Key|LeftMouseButton` :consume false
  (params (Key :type "Key Structure"))
  (:`Pressed`
    (bind _returnvalue (`self.Check Can Fire`))
    (if _returnvalue
      (bind _rpm_delay (`self.Calculate RPM`))
      (`/Game/_Game/GameObjects/Weapons/Ranged/Blueprints/BPML_Helpers.Delayed Loop` (`self.Ammo Use`) (`.Ammo_9_E518D3CB4D86DFD0FE1DB4B8A9009B40` (break `/Game/_Game/GameObjects/Weapons/SRT_Weapon` (`self.Stats`))) _rpm_delay :!label _label
        (:`Out`
          (`self.Fire`)))))
  (:`Released`
    (goto _label :!via `Break`)))

(fn `Calculate RPM`
  (returns (`RPM Delay` :type "Float (double-precision)"))
  (return (/ 1.0 (`.RPM_21_534CC3A64C2FA0DA5D74E2B22CE2E789` (break `/Game/_Game/GameObjects/Weapons/SRT_Weapon` (`self.Stats`))))))

(fn `Check Can Fire`
  (returns (ReturnValue :type Boolean))
  (bind ((`Ammo_9_E518D3CB4D86DFD0FE1DB4B8A9009B40` _ammo) (`IsEquipped?_22_A6061ACD41B6029BBB815683C1C1258F` _isequipped_)) (break `/Game/_Game/GameObjects/Weapons/SRT_Weapon` (`self.Stats`)))
  (return (and (<= (`self.Ammo Use`) _ammo) _isequipped_)))

(fn `Fire`
  (bind _returnvalue (`SceneComponent.K2_GetComponentLocation` (`self.Weapon`)))
  (`self.Increment Ammo Use`)
  (bind _outhit (`KismetSystemLibrary.BoxTraceSingle` :`Start` _returnvalue :`End` (+ _returnvalue (* (`KismetMathLibrary.GetForwardVector` (`SceneComponent.K2_GetComponentRotation` (`self.Weapon`))) (`.Range_7_ADFE3A0348974133F742FD8A6574BFD3` (break `/Game/_Game/GameObjects/Weapons/SRT_Weapon` (`self.Stats`))))) :`HalfSize` (* (`KismetMathLibrary.Vector_One`) (`.Area_13_73920EB942267A2CC9774C8DC1962BF6` (break `/Game/_Game/GameObjects/Weapons/SRT_Weapon` (`self.Stats`)))) :`TraceChannel` "TraceTypeQuery1" :`DrawDebugType` "ForOneFrame"))
  (bind _asbpa_base_enemy (cast `/Game/_Game/GameObjects/Enemies/Dummy/BPA_BaseEnemy` (`.HitActor` (`GameplayStatics.BreakHitResult` _outhit))))
  (`/Game/_Game/GameObjects/Enemies/Dummy/BP_TargetDummy.Hit` _asbpa_base_enemy (`.Damage_8_183C89F74114DFF6259EAEACAF91E0C2` (break `/Game/_Game/GameObjects/Weapons/SRT_Weapon` (`self.Stats`)))))

(fn `Increment Ammo Use`
  (bind _ammo_use (`self.Ammo Use`))
  (bind (_stats_range _stats_damage _stats_ammo) (break `/Game/_Game/GameObjects/Weapons/SRT_Weapon` (`self.Stats`)))
  (if (<= _ammo_use _stats_ammo)
    (set `self.Ammo Use` (+ _ammo_use 1)))
  (return))

(fn `Set Base Stats`
  (params (Equipped :type Boolean))
  (set `self.Stats` (make `/Game/_Game/GameObjects/Weapons/SRT_Weapon` 1000.0 5 12 10.0 1.0 Equipped))
  (set `self.Ammo Use` 1))

(fn `UserConstructionScript`)