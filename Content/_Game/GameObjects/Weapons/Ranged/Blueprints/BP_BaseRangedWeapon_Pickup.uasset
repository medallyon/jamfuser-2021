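; Base pickup actor for ranged weapons that lets the player equip the weapon it holds.
; Overlap begin enables interaction and shows a hint widget, and overlap end disables it and removes the widget.
; Pressing E while interaction is allowed passes the weapon child actor's class to the player character's Equip, then destroys the pickup.
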(event `Key|E` :consume false
  (params (Key :type "Key Structure"))
  (:`Pressed`
    (if (`self.Can Interact?`)
      (`self.PickUp`))))

(event `self.ReceiveActorBeginOverlap`
  (params (OtherActor :type "Actor Object Reference"))
  ;[0 0.9062 1] Interaction Hint
  (set `self.Can Interact?` true)
  (bind _returnvalue (`|CreateWidget` "/Game/_Game/UI/Widgets/HUD/WBP_InteractionHint.WBP_InteractionHint_C"))
  (bind _output_get (set `self.Interaction Widget Hint` _returnvalue))
  (`UserWidget.AddToViewport` _output_get 0))

(event `self.ReceiveActorEndOverlap`
  (params (OtherActor :type "Actor Object Reference"))
  ;[0 0.9062 1] Interaction Hint
  (`self.Hide Interaction Widget`))

(fn `PickUp`
  (`self.Hide Interaction Widget`)
  (bind _asworking_base_character_bp (cast `/Game/_Game/GameObjects/Character/Working/Working_Base_CharacterBP` (`GameplayStatics.GetPlayerCharacter` 0)))
  (`/Game/_Game/GameObjects/Character/Working/Working_Base_CharacterBP.Equip` _asworking_base_character_bp (`ChildActorComponent.ChildActorClass` (`self.BP_BaseRangedWeapon_Item`)))
  (`self.K2_DestroyActor`))

(fn `UserConstructionScript`)