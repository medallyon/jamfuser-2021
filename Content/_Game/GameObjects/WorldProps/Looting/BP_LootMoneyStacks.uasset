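; BP_LootMoneyStacks is a lootable money prop that adds 50 to the player's Loot, then destroys itself.
; BeginPlay varies the visible stack mesh using separate random rolls, though the Stack01 branch cannot fire because RandomInteger(2) never returns 2.
; Box overlap shows a widget and polls Interact through Delay loops, filling the player's Unlock while held.
; Full Unlock activates StaticMeshComponent, whose activation event handles the payout.
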(event `self.ReceiveBeginPlay`
  (bind _returnvalue (`KismetMathLibrary.RandomInteger` 2))
  (bind _sm_prop_money_stack_02 (`self.SM_Prop_Money_Stack_02`))
  (bind _sm_prop_money_stack_01 (`self.SM_Prop_Money_Stack_01`))
  (`|ExecutionSequence`
    (:`then_0`
      (if (== _returnvalue 0)
        (`SceneComponent.SetVisibility` _sm_prop_money_stack_01 false false)
        (`SceneComponent.SetVisibility` _sm_prop_money_stack_02 false false)
        (`SceneComponent.SetVisibility` (`self.SM_Prop_Money_Stack_03`) true false)))
    (:`then_1`
      (if (== _returnvalue 1)
        (`SceneComponent.SetVisibility` _sm_prop_money_stack_01 false false)
        (`SceneComponent.SetVisibility` (`self.SM_Prop_Money_Stack_03`) false false)
        (`SceneComponent.SetVisibility` _sm_prop_money_stack_02 true false)))
    (:`then_2`
      (if (== _returnvalue 2)
        (`SceneComponent.SetVisibility` _sm_prop_money_stack_02 false false)
        (`SceneComponent.SetVisibility` (`self.SM_Prop_Money_Stack_03`) false false)
        (`SceneComponent.SetVisibility` _sm_prop_money_stack_01 true false)))
    (:`then_3`
      (`SceneComponent.SetVisibility` (`self.Widget`) false false))))

(event `self.Box.OnComponentBeginOverlap`
  (params (OverlappedComponent :type "PrimitiveComponent Object Reference") (OtherActor :type "Actor Object Reference") (OtherComp :type "PrimitiveComponent Object Reference") (OtherBodyIndex :type Integer) (bFromSweep :type Boolean) (SweepResult :type "HitResult Structure (by ref)"))
  (bind _asbp_player (cast `/Game/_Game/GameObjects/Character/Blueprints/BP_Player` OtherActor))
  (set `/Game/_Game/GameObjects/Character/Blueprints/BP_Player.Unlock` 0.0 _asbp_player)
  (set `self.Overlapped` true)
  (if (`self.Overlapped`) :!label _label
    (bind _asbp_player_2 (cast `/Game/_Game/GameObjects/Character/Blueprints/BP_Player` OtherActor))
    (`SceneComponent.SetVisibility` (`self.Widget`) true false)
    (if (`/Game/_Game/GameObjects/Character/Blueprints/BP_Player.Interact` _asbp_player_2) :!label _label_2
      (bind _unlock (`/Game/_Game/GameObjects/Character/Blueprints/BP_Player.Unlock` _asbp_player_2))
      (if (>= _unlock 1.0)
        (`ActorComponent.Activate` (`self.StaticMeshComponent`) false)
        (else
          (set `/Game/_Game/GameObjects/Character/Blueprints/BP_Player.Unlock` (+ _unlock 0.33) _asbp_player_2)
          (`KismetSystemLibrary.Delay` 0.1)
          (goto _label_2)))
      (else
        (`KismetSystemLibrary.Delay` 0.05)
        (set `/Game/_Game/GameObjects/Character/Blueprints/BP_Player.Unlock` 0.0 _asbp_player_2)
        (goto _label)))))

(event `self.Box.OnComponentEndOverlap`
  (params (OverlappedComponent :type "PrimitiveComponent Object Reference") (OtherActor :type "Actor Object Reference") (OtherComp :type "PrimitiveComponent Object Reference") (OtherBodyIndex :type Integer))
  (set `self.Overlapped` false)
  (`SceneComponent.SetVisibility` (`self.Widget`) false false))

(event `self.StaticMeshComponent.OnComponentActivated`
  (params (Component :type "ActorComponent Object Reference") (bReset :type Boolean))
  (`SceneComponent.SetVisibility` (`self.SM_Prop_Money_Stack_01`) false false)
  (`SceneComponent.SetVisibility` (`self.SM_Prop_Money_Stack_02`) false false)
  (`SceneComponent.SetVisibility` (`self.SM_Prop_Money_Stack_03`) false false)
  (`PrimitiveComponent.SetCollisionEnabled` (`self.Box`) "NoCollision")
  (bind _asbp_player (cast `/Game/_Game/GameObjects/Character/Blueprints/BP_Player` (`GameplayStatics.GetPlayerCharacter` 0)))
  (set `/Game/_Game/GameObjects/Character/Blueprints/BP_Player.Loot` (+ (`/Game/_Game/GameObjects/Character/Blueprints/BP_Player.Loot` _asbp_player) 50) _asbp_player)
  (`self.K2_DestroyActor`))

(fn `UserConstructionScript`)