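; BP_HidingDrawer is a world prop that lets the player hide when interacting inside its trigger box.
; Box overlap creates an ALS_HUD widget for any overlapping actor, then casts that actor to BP_Player.
; A short Delay loop polls the player's Interact flag while overlapped, then sets Hiding and removes the widget.
; End overlap clears the overlap flag and removes the widget, but leaves Hiding untouched.
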(event `self.Box.OnComponentBeginOverlap`
  (params (OverlappedComponent :type "PrimitiveComponent Object Reference") (OtherActor :type "Actor Object Reference") (OtherComp :type "PrimitiveComponent Object Reference") (OtherBodyIndex :type Integer) (bFromSweep :type Boolean) (SweepResult :type "HitResult Structure (by ref)"))
  (set `self.Overlapped` true)
  (bind _returnvalue (`|CreateWidget` "/Game/AdvancedLocomotionV4/Blueprints/UI/ALS_HUD.ALS_HUD_C" (`GameplayStatics.GetPlayerController` 0)))
  (`UserWidget.AddToViewport` _returnvalue 0)
  (if (`self.Overlapped`) :!label _label
    (bind _asbp_player (cast `/Game/_Game/GameObjects/Character/Blueprints/BP_Player` OtherActor))
    (if (`/Game/_Game/GameObjects/Character/Blueprints/BP_Player.Interact` _asbp_player)
      (set `/Game/_Game/GameObjects/Character/Blueprints/BP_Player.Hiding` true _asbp_player)
      (`Widget.RemoveFromParent` _returnvalue)
      (else
        (`KismetSystemLibrary.Delay` 0.05)
        (goto _label)))))

(event `self.Box.OnComponentEndOverlap`
  (params (OverlappedComponent :type "PrimitiveComponent Object Reference") (OtherActor :type "Actor Object Reference") (OtherComp :type "PrimitiveComponent Object Reference") (OtherBodyIndex :type Integer))
  (set `self.Overlapped` false)
  (`Widget.RemoveFromParent` (stale `self.Box.OnComponentBeginOverlap` _returnvalue)))

(fn `UserConstructionScript`)