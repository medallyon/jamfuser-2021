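; BP_RifleTable is a world prop that lets the player choose the M4A1 rifle as their weapon.
; Entering its Box shows a widget and leaving hides it.
; While overlapped, a 0.05-second Delay loop polls the player's Interact flag instead of binding input.
; Once the flag is true, it writes BP_M4A1 and a weapon texture to BP_Player and stops polling.
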(event `self.ReceiveBeginPlay`
  (set `self.Overlapped` false)
  (`SceneComponent.SetVisibility` (`self.Widget`) false false))

(event `self.Box.OnComponentBeginOverlap`
  (params (OverlappedComponent :type "PrimitiveComponent Object Reference") (OtherActor :type "Actor Object Reference") (OtherComp :type "PrimitiveComponent Object Reference") (OtherBodyIndex :type Integer) (bFromSweep :type Boolean) (SweepResult :type "HitResult Structure (by ref)"))
  (`SceneComponent.SetVisibility` (`self.Widget`) true false)
  (set `self.Overlapped` true)
  (if (`self.Overlapped`) :!label _label
    (bind _asbp_player (cast `/Game/_Game/GameObjects/Character/Blueprints/BP_Player` OtherActor))
    (`SceneComponent.SetVisibility` (`self.Widget`) true false)
    (if (`/Game/_Game/GameObjects/Character/Blueprints/BP_Player.Interact` _asbp_player)
      (set `/Game/_Game/GameObjects/Character/Blueprints/BP_Player.Chosen Weapon` "/Game/_Game/GameObjects/Character/BP_M4A1.BP_M4A1_C" _asbp_player)
      (set `/Game/_Game/GameObjects/Character/Blueprints/BP_Player.WepTexture` "/Game/AdvancedLocomotionV4/Blueprints/UI/Arrow.Arrow" _asbp_player)
      (else
        (`KismetSystemLibrary.Delay` 0.05)
        (goto _label)))))

(event `self.Box.OnComponentEndOverlap`
  (params (OverlappedComponent :type "PrimitiveComponent Object Reference") (OtherActor :type "Actor Object Reference") (OtherComp :type "PrimitiveComponent Object Reference") (OtherBodyIndex :type Integer))
  (set `self.Overlapped` false)
  (`SceneComponent.SetVisibility` (`self.Widget`) false false))

(fn `UserConstructionScript`)