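; Player character with cursor-driven movement: holding right mouse moves it toward the point under the cursor.
; Each tick it turns the Player component's yaw to face the cursor hit.
; It switches the ABP_Robber Actions state while moving and on nearing the destination.
; ChangeCamera toggles the camera between its saved relative transform and the home base layout's CameraPointingOnScreen location at zero rotation.
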(event `self.ReceiveBeginPlay`
  ;[0 0.25 1] Set Initial Vars
  (set `PlayerController.bShowMouseCursor` true (`GameplayStatics.GetPlayerController` 0))
  (set `self.Camera Location` (`SceneComponent.RelativeLocation` (`self.Camera`)))
  (set `self.Camera Rotation` (`SceneComponent.RelativeRotation` (`self.Camera`))))

(event `Key|RightMouseButton`
  (params (Key :type "Key Structure"))
  ;[0 0.03906 1] Check Mouse Down
  (:`Pressed`
    (set `self.Is Mouse Down?` true))
  (:`Released`
    (set `self.Is Mouse Down?` false)))

(event `self.ReceiveTick`
  (params (DeltaSeconds :type "Float (single-precision)"))
  (bind _returnvalue (`GameplayStatics.GetPlayerController` 0))
  (bind (_returnvalue_roll _returnvalue_pitch) (`KismetMathLibrary.BreakRotator` (`self.K2_GetActorRotation`)))
  (bind (_returnvalue_roll_2 _returnvalue_pitch_2 _returnvalue_yaw) (`KismetMathLibrary.BreakRotator` (`KismetMathLibrary.FindLookAtRotation` (`self.K2_GetActorLocation`) (`.Location` (`GameplayStatics.BreakHitResult` (`PlayerController.GetHitResultUnderCursorByChannel` (`GameplayStatics.GetPlayerController` 0) "TraceTypeQuery1" true))))))
  ;[1 0.75 0] Rotate Character
  (`|ExecutionSequence`
    (:`then_0`
      ;[0 0.3437 1] Character Movement
      (if (`self.Is Mouse Down?`)
        (bind _output_get (set `self.Destination` (`.Location` (`GameplayStatics.BreakHitResult` (`PlayerController.GetHitResultUnderCursorByChannel` _returnvalue "TraceTypeQuery1" true)))))
        (`AIBlueprintHelperLibrary.SimpleMoveToLocation` _returnvalue _output_get)
        (set `self.Actions` "NewEnumerator0")
        ;[0.125 0 1] Animation Controller
        (bind _asabp_robber (cast `/Game/_Game/Character/ABP_Robber` (`SkeletalMeshComponent.GetAnimInstance` (`self.Player`)) :!label _label))
        (set `/Game/_Game/Character/ABP_Robber.Actions` (`self.Actions`) _asabp_robber)
        (elif (== (`self.Destination`) (`SceneComponent.K2_GetComponentLocation` (`self.Player`)) :`ErrorTolerance` 50.0)
          (set `self.Actions` "NewEnumerator1")
          (goto _label))))
    (:`then_1`
      (`SceneComponent.K2_SetWorldRotation` (`self.Player`) (`KismetMathLibrary.MakeRotator` _returnvalue_roll _returnvalue_pitch (+ _returnvalue_yaw -90.0)) false false))))

(fn `Change Camera`
  (if (not (== (`SceneComponent.K2_GetComponentRotation` (`self.Camera`)) (struct) :`ErrorTolerance` 0.1))
    (bind _returnvalue (`GameplayStatics.GetActorOfClass` "/Game/_Game/Base/BP_Home_Base_Combined_Layout.BP_Home_Base_Combined_Layout_C"))
    (`SceneComponent.K2_SetWorldLocationAndRotation` :`self` (`self.Camera`) :`NewLocation` (`SceneComponent.K2_GetComponentLocation` (`/Game/_Game/Base/BP_Home_Base_Combined_Layout.Camera Pointing On Screen` _returnvalue)))
    (else
      (`SceneComponent.K2_SetRelativeLocationAndRotation` (`self.Camera`) (`self.Camera Location`) (`self.Camera Rotation`) false false))))

(fn `UserConstructionScript`)