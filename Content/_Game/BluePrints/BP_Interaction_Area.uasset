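; BP_Interaction_Area is a trigger area that lets the player switch camera by pressing E while inside it.
; Overlap with BP_Player sets the CanIteract flag and adds a WBP_Interaction_Hint widget to the viewport, and leaving clears both.
; The E key handler checks that flag, then finds BP_Player with GetActorOfClass and calls its ChangeCamera function.
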(event `Key|E`
  (params (Key :type "Key Structure"))
  ;[0.9453 1 0] ReFocus Camera
  (:`Pressed`
    (if (`self.Can Iteract?`)
      (bind _returnvalue (`GameplayStatics.GetActorOfClass` "/Game/_Game/Character/BP_Player.BP_Player_C"))
      (`/Game/_Game/Character/BP_Player.Change Camera` _returnvalue))))

(event `self.ReceiveActorBeginOverlap`
  (params (OtherActor :type "Actor Object Reference"))
  ;[0 0.9062 1] Interaction Hint
  (cast `/Game/_Game/Character/BP_Player` OtherActor)
  (set `self.Can Iteract?` true)
  (bind _returnvalue (`|CreateWidget` "/Game/_Game/Widgets/WBP_Interaction_Hint.WBP_Interaction_Hint_C"))
  (`UserWidget.AddToViewport` _returnvalue 0))

(event `self.ReceiveActorEndOverlap`
  (params (OtherActor :type "Actor Object Reference"))
  ;[0 0.9062 1] Interaction Hint
  (cast `/Game/_Game/Character/BP_Player` OtherActor)
  (set `self.Can Iteract?` false)
  (`Widget.RemoveFromParent` (stale `self.ReceiveActorBeginOverlap` _returnvalue)))

(fn `UserConstructionScript`)